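; Health pickup that heals an overlapping Bogo_Player_Character with a nonzero player number, capped at starting health.
; On pickup it updates that player's HUD, plays a sound and disables itself until a delay re-enables it.
; Tick spins the pack, bobs it with a sine offset applied each frame, and syncs both cube meshes' visibility to the enabled flag.
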(event OnComponentBeginOverlap(Collision)
  (params (OverlappedComponent :type Primitive%20Component%20Object%20Reference) (OtherActor :type Actor%20Object%20Reference) (OtherComp :type Primitive%20Component%20Object%20Reference) (OtherBodyIndex :type Integer) (bFromSweep :type Boolean) (SweepResult :type Hit%20Result%20Structure%20%28by%20ref%29))
  (if (Variables|Default|GetEnabled)
    (bind _asbogo_player_character (Utilities|Casting|CastToBogo_Player_Character OtherActor))
    (if (!= (Variables|/Game/Kyle_Stuff/Blueprints/Bogo_Player_Character.Bogo_Player_Character_C|GetPlayer%20Number _asbogo_player_character) 0)
      (bind _output_get (Variables|/Game/Kyle_Stuff/Blueprints/Bogo_Player_Character.Bogo_Player_Character_C|SetHealth _asbogo_player_character (Math|Float|Min(Float) (+ (Variables|/Game/Kyle_Stuff/Blueprints/Bogo_Player_Character.Bogo_Player_Character_C|GetHealth _asbogo_player_character) (Variables|Default|GetHealth)) (Variables|/Game/Kyle_Stuff/Blueprints/Bogo_Player_Character.Bogo_Player_Character_C|GetStarting%20Health _asbogo_player_character))))
      (Default|UpdateHealth (Variables|/Game/Kyle_Stuff/Blueprints/Bogo_Player_Character.Bogo_Player_Character_C|GetHUD _asbogo_player_character) (/ _output_get (Variables|/Game/Kyle_Stuff/Blueprints/Bogo_Player_Character.Bogo_Player_Character_C|GetStarting%20Health _asbogo_player_character)))
      (Audio|PlaySoundatLocation "/Game/Kyle_Stuff/Sounds/HealthGet.HealthGet" (Transformation|GetActorLocation) "0, 0, 0" 1.0 1.0 0.0 0 0 0 0)
      (Variables|Default|SetEnabled false)
      (Utilities|FlowControl|Delay (Variables|Default|GetDelay))
      (Variables|Default|SetEnabled true))))

(event EventBeginPlay
  (Transformation|AddActorWorldOffset (Math|Vector|MakeVector 0.0 0.0 (Variables|Default|GetAuto%20Offset))))

(event EventTick
  (params (DeltaSeconds :type Float%20%28single-precision%29))
  (bind _hover_speed (Variables|Default|GetHover%20Speed))
  (Class|Actor|AddActorWorldRotation (Math|Rotator|MakeRotator 0.0 0.0 (* (Variables|Default|GetRotate%20Speed) DeltaSeconds)))
  (bind _output_get (Variables|Default|SetTimer (+ DeltaSeconds (Variables|Default|GetTimer))))
  (Transformation|AddActorWorldOffset (Math|Vector|MakeVector 0.0 0.0 (* (Math|Trig|Sin(Degrees) (* _output_get (.x _hover_speed))) (.y _hover_speed))))
  (Rendering|SetVisibility (Variables|Default|GetCube2) (Variables|Default|GetEnabled) false))

(fn ConstructionScript)