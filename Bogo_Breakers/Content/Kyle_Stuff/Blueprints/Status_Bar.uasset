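; World-space status bar actor that shows a value as a percentage of a min/max range by X-scaling Value and Trail pivots.
; SetValue and SetReferences set the target; Tick lerps toward it by a fixed per-frame alpha, snapping when close or when lerping is off.
; With LerpTrail, the value jumps while the trail catches up.
; Helpers convert values, swap materials and face a target camera.
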(event EventTick
  (params (DeltaSeconds :type Float%20%28single-precision%29))
  (bind _targetvalue (Variables|Default|GetTargetValue))
  ;[0.5586 0.1968 1] Lerps the current value if it is able to be lerped
  (if (!= (Variables|Default|GetCurrentValue) (Variables|Default|GetTargetValue))
    (Variables|Default|SetCurrentValue (Math|Float|SelectFloat (Math|Float|SelectFloat (Math|Float|Lerp (Variables|Default|GetCurrentValue) _targetvalue (Variables|Default|GetLerpSpeed)) _targetvalue (Variables|Default|GetLerp)) _targetvalue (>= (Math|Float|Absolute(Float) (- _targetvalue (Variables|Default|GetCurrentValue))) 0.01)))
    (CallFunction|UpdateBar)))

(fn ConstructionScript)

(fn ChangeColor
  (params (NewColor :type Material%20Object%20Reference) (IsTrail :type Boolean))
  ;[0.5586 0.1968 1] Changes the color of a bar
  (Rendering|Material|SetMaterial (select IsTrail (Variables|Default|GetTrail) (Variables|Default|GetValue)) 0 NewColor))

(fn FaceCamera
  ;[0.5586 0.1968 1] Looks at the set camera
  (Transformation|SetActorRotation (Math|Conversions|RotationFromXVector (- (Transformation|GetActorLocation (Variables|Default|GetTargetCamera)) (Transformation|GetActorLocation)))))

(fn UpdateBar
  (bind _valuepivot (Variables|Default|GetValuePivot))
  (bind _trailpivot (Variables|Default|GetTrailPivot))
  (bind _currentvalue (Variables|Default|GetCurrentValue))
  (bind _relativescale3d (Variables|/Script/Engine.SceneComponent|GetRelativeScale3D _trailpivot))
  (bind _relativescale3d_2 (Variables|/Script/Engine.SceneComponent|GetRelativeScale3D _valuepivot))
  ;[0.5586 0.1968 1] Updates the bar based on the current value
  (if (Variables|Default|GetLerpTrail)
    (Transformation|SetRelativeScale3D _valuepivot (Math|Vector|MakeVector (Variables|Default|GetTargetValue) (.y _relativescale3d_2) (.z _relativescale3d_2)))
    (Transformation|SetRelativeScale3D _trailpivot (Math|Vector|MakeVector _currentvalue (.y _relativescale3d) (.z _relativescale3d)))
    (else
      (Transformation|SetRelativeScale3D _valuepivot (Math|Vector|MakeVector _currentvalue (.y _relativescale3d_2) (.z _relativescale3d_2)))
      (Transformation|SetRelativeScale3D _trailpivot (Math|Vector|MakeVector _currentvalue (.y _relativescale3d) (.z _relativescale3d))))))

(fn CalcPercentage
  (params (Value :type Float%20%28double-precision%29) (Min :type Float%20%28double-precision%29) (Max :type Float%20%28double-precision%29))
  ;[0.5586 0.1968 1] Calculates a percentage from a value
  (return (/ (- Value Min) (- Max Min))))

(fn CalcValue
  (params (Percentage :type Float%20%28double-precision%29) (Min :type Float%20%28double-precision%29) (Max :type Float%20%28double-precision%29))
  ;[0.5586 0.1968 1] Calculates a value from a percentage
  (return (+ (* (- Max Min) Percentage) Min)))

(fn SetValue
  (params (Percentage :type Float%20%28double-precision%29) (SkipLerp :type Boolean))
  ;[0.5586 0.1968 1] Updates the bar's value
  (Variables|Default|SetTargetValue Percentage)
  (if SkipLerp
    (Variables|Default|SetCurrentValue Percentage))
  (CallFunction|UpdateBar))

(fn SetReferences
  (params (CurrentValue :type Float%20%28double-precision%29) (Minimum :type Float%20%28double-precision%29) (Maximum :type Float%20%28double-precision%29) (SkipLerp :type Boolean))
  ;[0.5586 0.1968 1] Sets the bounds and current value of the bar
  (Variables|Default|SetRefValue CurrentValue)
  (Variables|Default|SetRefMinValue Minimum)
  (Variables|Default|SetRefMaxValue Maximum)
  (CallFunction|SetValue (CallFunction|GetPercentage CurrentValue) SkipLerp))

(fn GetPercentage
  (params (Value :type Float%20%28double-precision%29))
  ;[0.5586 0.1968 1] Gets a percentage of the bar from a given value
  (return (CallFunction|CalcPercentage Value (Variables|Default|GetRefMinValue) (Variables|Default|GetRefMaxValue))))

(fn GetValue
  (params (Percentage :type Float%20%28double-precision%29))
  ;[0.5586 0.1968 1] Gets a value of the bar from a given percentage
  (return (CallFunction|CalcValue Percentage (Variables|Default|GetRefMinValue) (Variables|Default|GetRefMaxValue))))