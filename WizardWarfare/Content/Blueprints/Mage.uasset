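; Mage enemy that stands in place, turns to face the player when in range and periodically fires DarkMagicAttack projectiles.
; Tick drives a frame-counted attack cooldown, idle/attack animation switching, damage-flash material reset, and death with a Mana pickup drop.
; Overlap tags set damage for Magic, Thunder and Fire hits.
; Death, or Freeze when the player's FrozenEnemy slot is empty (then set to 3), removes the mage without a drop via a -100 Health sentinel.
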(event OnComponentBeginOverlap(Overlap)
  (params (OverlappedComponent :type Primitive%20Component%20Object%20Reference) (OtherActor :type Actor%20Object%20Reference) (OtherComp :type Primitive%20Component%20Object%20Reference) (OtherBodyIndex :type Integer) (bFromSweep :type Boolean) (SweepResult :type Hit%20Result%20Structure%20%28by%20ref%29))
  (bind _mesh (Variables|Character|GetMesh))
  ;[1 1 1] Damage + Freeze
  (if (Components|ComponentHasTag OtherComp "Death")
    (Variables|Default|SetHealth -100 :!label _label)
    (else
      (bind _asbp_third_person_character (Utilities|Casting|CastToBP_ThirdPersonCharacter (Game|GetPlayerCharacter 0)))
      (if (Components|ComponentHasTag OtherComp "Freeze")
        (if (== (Variables|/Game/Blueprints/BP_ThirdPersonCharacter.BP_ThirdPersonCharacter_C|GetFrozenEnemy _asbp_third_person_character) 0)
          (Variables|/Game/Blueprints/BP_ThirdPersonCharacter.BP_ThirdPersonCharacter_C|SetFrozenEnemy _asbp_third_person_character 3)
          (Variables|/Game/Blueprints/BP_ThirdPersonCharacter.BP_ThirdPersonCharacter_C|SetMana _asbp_third_person_character (+ (Variables|/Game/Blueprints/BP_ThirdPersonCharacter.BP_ThirdPersonCharacter_C|GetMana _asbp_third_person_character) 0.0))
          (goto _label)
          (else
            _)))
      (if (Actor|ActorHasTag OtherActor "Magic")
        (Variables|Default|SetHealth (- (Variables|Default|GetHealth) 1))
        (Rendering|Material|SetMaterial _mesh 0 "/Game/Materials/Characters/Damage_Mage.Damage_Mage" :!label _label_2)
        (Rendering|Material|SetMaterial _mesh 1 "/Game/Materials/Characters/Damage_Mage.Damage_Mage")
        (Variables|Default|SetDamageFlash 0)
        (elif (Actor|ActorHasTag OtherActor "Thunder")
          (Variables|Default|SetHealth (- (Variables|Default|GetHealth) 2))
          (goto _label_2)
          (elif (Actor|ActorHasTag OtherActor "Fire")
            (Variables|Default|SetHealth (- (Variables|Default|GetHealth) 4))
            (goto _label_2)))))))

(event EventBeginPlay
  ;[1 1 1] Enemy AI
  (Pawn|SpawnDefaultController))

(event EventTick
  (params (DeltaSeconds :type Float%20%28single-precision%29))
  (bind _capsulecomponent (Variables|Collision|GetCapsuleComponent))
  (bind _mesh (Variables|Character|GetMesh))
  (bind _mesh_2 (Variables|Character|GetMesh))
  (bind _returnvalue (Transformation|GetWorldLocation _capsulecomponent))
  ;[1 1 1] Enemy AI
  (Variables|Default|SetDamageFlash (+ (Variables|Default|GetDamageFlash) 1))
  (if (> (Variables|Default|GetDamageFlash) 3)
    (Rendering|Material|SetMaterial _mesh 0 "/Game/Assets/CityofBrass_Enemies/Materials/Wizard_Inst.Wizard_Inst")
    (Rendering|Material|SetMaterial _mesh 1 "/Game/Assets/CityofBrass_Enemies/Materials/FermaleWarrior_Inst.FermaleWarrior_Inst"))
  (if (<= (Variables|Default|GetHealth) 0)
    (if (== (Variables|Default|GetHealth) -100)
      _
      (else
        (Game|SpawnActorfromClass "/Game/Blueprints/Mana.Mana_C" (Math|Conversions|ToTransform(Vector) _returnvalue) "Undefined" 0 0)))
    (Actor|DestroyActor)
    (else
      (bind _asbp_third_person_character (Utilities|Casting|CastToBP_ThirdPersonCharacter (Game|GetPlayerCharacter 0)))
      (if (< (Math|Vector|Distance(Vector) _returnvalue (Transformation|GetWorldLocation (Variables|/Script/Engine.Character|GetMesh _asbp_third_person_character))) 2.1e+03)
        (Transformation|SetActorRotation (Math|Rotator|MakeRotator 0.0 0.0 (.Yaw (Math|Rotator|BreakRotator (Math|Rotator|FindLookatRotation _returnvalue (Transformation|GetWorldLocation (Variables|/Script/Engine.Character|GetMesh _asbp_third_person_character)))))))
        (if (> (Variables|Default|GetAttackCooldown) 16)
          (Game|SpawnActorfromClass "/Game/Blueprints/DarkMagicAttack.DarkMagicAttack_C" (Math|Transform|MakeTransform (Transformation|GetWorldLocation (Variables|Default|GetAttackSpawn)) (Math|Rotator|FindLookatRotation _returnvalue (Transformation|GetWorldLocation (Variables|/Script/Engine.Character|GetMesh _asbp_third_person_character)))) "Undefined" 0 0)
          (Variables|Default|SetAttackCooldown 0)
          (else
            (Variables|Default|SetAttackCooldown (+ (Variables|Default|GetAttackCooldown) 1))))
        (if (not (== (Variables|Default|GetAnimation) 1))
          (Components|Animation|PlayAnimation _mesh_2 "/Game/Assets/CityofBrass_Enemies/Meshes/Enemy/Corpse/animation/Corpse_Alert_Attack_Push.Corpse_Alert_Attack_Push" true)
          (Variables|Default|SetAnimation 1)
          (Variables|/Script/Engine.SkeletalMeshComponent|SetGlobalAnimRateScale _mesh_2 1.2))
        (elif (not (== (Variables|Default|GetAnimation) 0))
          (Components|Animation|PlayAnimation _mesh_2 "/Game/Assets/CityofBrass_Enemies/Meshes/Enemy/Corpse/animation/Corpse_alert_idle.Corpse_alert_idle" true)
          (Variables|Default|SetAnimation 0)
          (Variables|/Script/Engine.SkeletalMeshComponent|SetGlobalAnimRateScale _mesh_2 1.0))))))

(fn ConstructionScript)