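; FireAttack is a flamethrower attack actor that stays active while the player holds the left mouse button.
; Each tick it snaps to BP_ThirdPersonCharacter's PlayerXYZ and camera rotation, and spins its Collision component by stepping the relative pitch with a wraparound.
; It destroys itself when the button is released or the character's mana runs too low.
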(event EventTick
  (params (DeltaSeconds :type Float%20%28single-precision%29))
  (bind _collision (Variables|Default|GetCollision))
  (bind _relativerotation (Variables|/Script/Engine.SceneComponent|GetRelativeRotation _collision))
  (bind (_roll _pitch _yaw) (Math|Rotator|BreakRotator _relativerotation))
  ;[1 1 1] Flamethrower (destroy on releasing LMB)
  (bind _asbp_third_person_character (Utilities|Casting|CastToBP_ThirdPersonCharacter (Game|GetPlayerCharacter 0)))
  ;[1 1 1] Hover With Staff + Rotate
  (Transformation|SetActorLocationAndRotation (+ (Variables|/Game/Blueprints/BP_ThirdPersonCharacter.BP_ThirdPersonCharacter_C|GetPlayerXYZ _asbp_third_person_character) "") (Variables|/Game/Blueprints/BP_ThirdPersonCharacter.BP_ThirdPersonCharacter_C|GetCameraRotation _asbp_third_person_character))
  (if (>= _pitch 3.5e+02)
    (Transformation|SetRelativeRotation _collision (Math|Rotator|MakeRotator _roll 0.0 _yaw) false false))
  (Transformation|SetRelativeRotation _collision (Math|Rotator|MakeRotator _roll (+ _pitch 5e+01) _yaw) false false)
  (if (Variables|/Game/Blueprints/BP_ThirdPersonCharacter.BP_ThirdPersonCharacter_C|GetLeftMouseHeld? _asbp_third_person_character)
    (if (not (> (Variables|/Game/Blueprints/BP_ThirdPersonCharacter.BP_ThirdPersonCharacter_C|GetMana _asbp_third_person_character) 3.0))
      (Actor|DestroyActor :!label _label))
    (else
      (goto _label))))

(fn ConstructionScript)