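; Gate actor that lowers itself once the third-person player character holds the key.
; Every tick it casts the player to BP_ThirdPersonCharacter and checks its Key flag.
; With the key, the mesh steps down along Z each frame, frame-rate dependent, until it reaches a floor height.
; Without the key, it snaps back to a hard-coded closed world position.
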(event EventTick
  (params (DeltaSeconds :type Float%20%28single-precision%29))
  (bind _staticmesh (Variables|Default|GetStaticMesh))
  (bind _staticmesh_2 (Variables|Default|GetStaticMesh))
  (bind _returnvalue (Transformation|GetWorldLocation _staticmesh_2))
  (bind (_x _y _z) (Class|KismetMathLibrary|BreakVector3f _returnvalue))
  ;[1 1 1] Open Gate
  (bind _asbp_third_person_character (Utilities|Casting|CastToBP_ThirdPersonCharacter (Game|GetPlayerCharacter 0)))
  (if (Variables|/Game/Blueprints/BP_ThirdPersonCharacter.BP_ThirdPersonCharacter_C|GetKey? _asbp_third_person_character)
    (if (> _z 2.3e+02)
      (Transformation|SetWorldLocation _staticmesh (Math|Vector|MakeVector _x _y (- _z 4.0)) false false))
    (else
      (Transformation|SetWorldLocation _staticmesh "7100.000000,-700.000000,730.000000" false false))))

(fn ConstructionScript)