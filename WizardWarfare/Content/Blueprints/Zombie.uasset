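; Zombie enemy that turns and walks toward the player when within range, attacks up close on a cooldown, and idles otherwise.
; Tick drives the AI, animation switching, tick-counted cooldown and hit flash, and death, which drops a Mana pickup.
; Overlap tags apply Magic, Thunder or Fire damage.
; Death, or Freeze while the player's FrozenEnemy is unset, sets a sentinel health that removes the zombie without a drop.
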(event OnComponentBeginOverlap(Overlap)
  (params (OverlappedComponent :type Primitive%20Component%20Object%20Reference) (OtherActor :type Actor%20Object%20Reference) (OtherComp :type Primitive%20Component%20Object%20Reference) (OtherBodyIndex :type Integer) (bFromSweep :type Boolean) (SweepResult :type Hit%20Result%20Structure%20%28by%20ref%29))
  ;[1 1 1] Damage + Freeze
  (if (Components|ComponentHasTag OtherComp "Death")
    (Variables|Default|SetHealth -100 :!label _label)
    (else
      (bind _asbp_third_person_character (Utilities|Casting|CastToBP_ThirdPersonCharacter (Game|GetPlayerCharacter 0)))
      (if (Components|ComponentHasTag OtherComp "Freeze")
        (if (== (Variables|/Game/Blueprints/BP_ThirdPersonCharacter.BP_ThirdPersonCharacter_C|GetFrozenEnemy _asbp_third_person_character) 0)
          (Variables|/Game/Blueprints/BP_ThirdPersonCharacter.BP_ThirdPersonCharacter_C|SetFrozenEnemy _asbp_third_person_character 1)
          (Variables|/Game/Blueprints/BP_ThirdPersonCharacter.BP_ThirdPersonCharacter_C|SetMana _asbp_third_person_character (+ (Variables|/Game/Blueprints/BP_ThirdPersonCharacter.BP_ThirdPersonCharacter_C|GetMana _asbp_third_person_character) 0.0))
          (goto _label)
          (else
            _)))
      (if (Actor|ActorHasTag OtherActor "Magic")
        (Variables|Default|SetHealth (- (Variables|Default|GetHealth) 1))
        (Rendering|Material|SetMaterial (Variables|Character|GetMesh) 0 "/Game/Materials/Characters/Damage.Damage" :!label _label_2)
        (Variables|Default|SetDamageFlash 0)
        (elif (Actor|ActorHasTag OtherActor "Thunder")
          (Variables|Default|SetHealth (- (Variables|Default|GetHealth) 2))
          (goto _label_2)
          (elif (Actor|ActorHasTag OtherActor "Fire")
            (Variables|Default|SetHealth (- (Variables|Default|GetHealth) 4))
            (goto _label_2)))))))

(event EventBeginPlay
  ;[1 1 1] Enemy AI
  (Pawn|SpawnDefaultController))

(event EventTick
  (params (DeltaSeconds :type Float%20%28single-precision%29))
  (bind _capsulecomponent (Variables|Collision|GetCapsuleComponent))
  (bind _mesh (Variables|Character|GetMesh))
  (bind _returnvalue (Transformation|GetWorldLocation _capsulecomponent))
  ;[1 1 1] Enemy AI
  (Variables|Default|SetAttackCooldown (+ (Variables|Default|GetAttackCooldown) 1))
  (Variables|Default|SetDamageFlash (+ (Variables|Default|GetDamageFlash) 1))
  (if (> (Variables|Default|GetDamageFlash) 2)
    (Rendering|Material|SetMaterial (Variables|Character|GetMesh) 0 "/Game/Assets/CityofBrass_Enemies/Materials/Large_Inst.Large_Inst"))
  (if (<= (Variables|Default|GetHealth) 0)
    (if (== (Variables|Default|GetHealth) -100)
      _
      (else
        (Game|SpawnActorfromClass "/Game/Blueprints/Mana.Mana_C" (Math|Conversions|ToTransform(Vector) _returnvalue) "Undefined" 0 0)))
    (Actor|DestroyActor)
    (else
      (bind _asbp_third_person_character (Utilities|Casting|CastToBP_ThirdPersonCharacter (Game|GetPlayerCharacter 0)))
      (if (< (Math|Vector|Distance(Vector) _returnvalue (Transformation|GetWorldLocation (Variables|/Script/Engine.Character|GetMesh _asbp_third_person_character))) 1e+03)
        (if (> (Math|Vector|Distance(Vector) _returnvalue (Transformation|GetWorldLocation (Variables|/Script/Engine.Character|GetMesh _asbp_third_person_character))) 2e+02)
          (Transformation|SetActorRotation (Math|Rotator|MakeRotator 0.0 0.0 (.Yaw (Math|Rotator|BreakRotator (Math|Rotator|FindLookatRotation _returnvalue (Transformation|GetWorldLocation (Variables|/Script/Engine.Character|GetMesh _asbp_third_person_character)))))))
          (Pawn|Input|AddMovementInput (Math|Vector|GetForwardVector (Variables|Collision|GetCapsuleComponent)) 0.5 false)
          (if (not (== (Variables|Default|GetAnimation) 0))
            (Components|Animation|PlayAnimation _mesh "/Game/Assets/CityofBrass_Enemies/Meshes/Enemy/Charger/Animation/Charger_Passive_Walk.Charger_Passive_Walk" true)
            (Variables|Default|SetAnimation 0)
            (Variables|/Script/Engine.SkeletalMeshComponent|SetGlobalAnimRateScale _mesh 1.5))
          (else
            (if (== (Variables|Default|GetAnimation) 2)
              _
              (else
                (Components|Animation|PlayAnimation _mesh "/Game/Assets/CityofBrass_Enemies/Meshes/Enemy/Corpse/animation/Corpse_Alert_Attack_Basic01.Corpse_Alert_Attack_Basic01" true)
                (Variables|Default|SetAnimation 2)
                (Variables|/Script/Engine.SkeletalMeshComponent|SetGlobalAnimRateScale _mesh 2.0)))
            (if (> (Variables|Default|GetAttackCooldown) 20)
              (Variables|/Game/Blueprints/BP_ThirdPersonCharacter.BP_ThirdPersonCharacter_C|SetHealth _asbp_third_person_character (- (Variables|/Game/Blueprints/BP_ThirdPersonCharacter.BP_ThirdPersonCharacter_C|GetHealth _asbp_third_person_character) 10))
              (Variables|Default|SetAttackCooldown 0)
              (Variables|/Game/Blueprints/BP_ThirdPersonCharacter.BP_ThirdPersonCharacter_C|SetDamageFlash _asbp_third_person_character 0))))
        (elif (not (== (Variables|Default|GetAnimation) 1))
          (Components|Animation|PlayAnimation _mesh "/Game/Assets/CityofBrass_Enemies/Meshes/Enemy/Charger/Animation/Charger_Passive_Ilde.Charger_Passive_Ilde" true)
          (Variables|Default|SetAnimation 1))))))

(fn ConstructionScript)