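; ThunderSpell is a pickup that grants the player the thunder spell.
; On overlap with the player character, it sets the Thunder flag and AttackSelection on BP_ThirdPersonCharacter, then destroys itself.
; Each tick it bobs its Collision component vertically by adding the sine of a looping time counter, advanced by a fixed step independent of frame time.
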(event EventTick
  (params (DeltaSeconds :type Float%20%28single-precision%29))
  (bind _collision (Variables|Default|GetCollision))
  (bind _returnvalue (Transformation|GetWorldLocation _collision))
  (bind (_x _y _z) (Class|KismetMathLibrary|BreakVector3f _returnvalue))
  ;[1 1 1] Levitation (using Sin)
  (Variables|Default|SetTime (+ (Variables|Default|GetTime) 0.1))
  (if (> (Variables|Default|GetTime) 1e+02)
    (Variables|Default|SetTime 0.0))
  (Transformation|SetWorldLocation (Variables|Default|GetCollision) (Math|Vector|MakeVector _x _y (+ _z (Math|Trig|Sin(Radians) (Variables|Default|GetTime)))) false false))

(event Collision|EventActorBeginOverlap
  (params (OtherActor :type Actor%20Object%20Reference))
  (bind _returnvalue (Game|GetPlayerCharacter 0))
  ;[1 1 1] Item Collision (Only with Player)
  (if (== OtherActor _returnvalue)
    (bind _asbp_third_person_character (Utilities|Casting|CastToBP_ThirdPersonCharacter _returnvalue))
    (Variables|/Game/Blueprints/BP_ThirdPersonCharacter.BP_ThirdPersonCharacter_C|SetThunder? _asbp_third_person_character true)
    (Variables|/Game/Blueprints/BP_ThirdPersonCharacter.BP_ThirdPersonCharacter_C|SetAttackSelection _asbp_third_person_character 2)
    (Actor|DestroyActor)))

(fn ConstructionScript)