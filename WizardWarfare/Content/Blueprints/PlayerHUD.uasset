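; PlayerHUD is a canvas HUD that shows the third-person character's health, mana, selected spell and crosshair.
; Each DrawHUD call reads BP_ThirdPersonCharacter, drawing health, then branching on AttackSelection for the colored spell label, mana and matching crosshair.
; Crosshairs for Magic Ball, Ice Block, Thunderbolt and Flamethrower are built from rectangles and shifted horizontally according to LeftShoulder.
; Dark offset duplicates give text and crosshair lines drop shadows.
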(event EventDrawHUD
  (params (SizeX :type Integer) (SizeY :type Integer))
  ;[1 1 1] HUD Script
  (Variables|Default|SetSize%20X (/ (Math|Conversions|ToFloat(Integer) SizeX) 2.0))
  (Variables|Default|SetSize%20Y (/ (Math|Conversions|ToFloat(Integer) SizeY) 2.0))
  (bind _asbp_third_person_character (Utilities|Casting|CastToBP_ThirdPersonCharacter (Game|GetPlayerCharacter 0)))
  ;[1 1 1] Health
  (HUD|DrawText (Utilities|String|ToString(Integer) (Variables|/Game/Blueprints/BP_ThirdPersonCharacter.BP_ThirdPersonCharacter_C|GetHealth _asbp_third_person_character)) "(R=0.000000,G=0.000000,B=0.000000,A=1.000000)" (+ (* SizeX 0.0) 52.0) (+ (* SizeY 1.0) -198.0) 0 3.5 false)
  (HUD|DrawText (Utilities|String|ToString(Integer) (Variables|/Game/Blueprints/BP_ThirdPersonCharacter.BP_ThirdPersonCharacter_C|GetHealth _asbp_third_person_character)) "(R=1.000000,G=0.000000,B=0.000000,A=1.000000)" (+ (* SizeX 0.0) 5e+01) (+ (* SizeY 1.0) -2e+02) 0 3.5 false)
  ;[1 1 1] Spells and Mana
  (if (== (Variables|/Game/Blueprints/BP_ThirdPersonCharacter.BP_ThirdPersonCharacter_C|GetAttackSelection _asbp_third_person_character) 0)
    (HUD|DrawText "(Q)     < 1. Magic Ball >     (E)" "(R=0.000000,G=0.000000,B=0.000000,A=1.000000)" (+ (Variables|Default|GetSize%20X) -135.0) (+ (* SizeY 0.0) 30) 0 2.0 false)
    (HUD|DrawText "(Q)     < 1. Magic Ball >     (E)" "(R=0.039546,G=0.921582,B=0.006512,A=1.000000)" (+ (Variables|Default|GetSize%20X) -137.0) (+ (* SizeY 0.0) 28) 0 2.0 false)
    (HUD|DrawText (Utilities|String|ToString(Integer) (Class|KismetMathLibrary|Round64 (Variables|/Game/Blueprints/BP_ThirdPersonCharacter.BP_ThirdPersonCharacter_C|GetMana _asbp_third_person_character))) "(R=0.000000,G=0.000000,B=0.000000,A=1.000000)" (+ (* SizeX 0.0) 52.0) (+ (* SizeY 1.0) -148.0) 0 3.5 false :!label _label)
    (HUD|DrawText (Utilities|String|ToString(Integer) (Class|KismetMathLibrary|Round64 (Variables|/Game/Blueprints/BP_ThirdPersonCharacter.BP_ThirdPersonCharacter_C|GetMana _asbp_third_person_character))) "(R=0.095307,G=0.791298,B=0.854993,A=1.000000)" (+ (* SizeX 0.0) 5e+01) (+ (* SizeY 1.0) -1.5e+02) 0 3.5 false)
    ;[1 1 1] Crosshair (Magic Attack)
    (if (== (Variables|/Game/Blueprints/BP_ThirdPersonCharacter.BP_ThirdPersonCharacter_C|GetAttackSelection _asbp_third_person_character) 0)
      (if (Variables|/Game/Blueprints/BP_ThirdPersonCharacter.BP_ThirdPersonCharacter_C|GetLeftShoulder? _asbp_third_person_character)
        (HUD|DrawRect "(R=0.000000,G=0.000000,B=0.000000,A=0.300000)" (+ (+ (Variables|Default|GetSize%20X) -10.5) 98.0) (+ (+ (Variables|Default|GetSize%20Y) 2.0) 0.0) 25.0 2.0)
        (HUD|DrawRect "(R=0.000000,G=0.000000,B=0.000000,A=0.300000)" (+ (+ (Variables|Default|GetSize%20X) 1.0) 98.0) (+ (+ (Variables|Default|GetSize%20Y) -1e+01) 0.0) 2.0 25.0)
        (HUD|DrawRect "(R=0.027451,G=0.913726,B=0.003922,A=0.301961)" (+ (+ (Variables|Default|GetSize%20X) -12.5) 98.0) (+ (+ (Variables|Default|GetSize%20Y) 0.0) 0.0) 25.0 2.0)
        (HUD|DrawRect "(R=0.027451,G=0.913726,B=0.003922,A=0.301961)" (+ (+ (Variables|Default|GetSize%20X) -1.0) 98.0) (+ (+ (Variables|Default|GetSize%20Y) -12.0) 0.0) 2.0 25.0)
        (HUD|DrawRect "(R=0.026241,G=0.913099,B=0.003677,A=1.000000)" (+ (+ (Variables|Default|GetSize%20X) -1.0) 98.0) (+ (+ (Variables|Default|GetSize%20Y) 0.0) 0.0) 2.0 2.0)
        (else
          (HUD|DrawRect "(R=0.000000,G=0.000000,B=0.000000,A=0.300000)" (+ (+ (Variables|Default|GetSize%20X) -10.5) -6e+01) (+ (+ (Variables|Default|GetSize%20Y) 2.0) 0.0) 25.0 2.0)
          (HUD|DrawRect "(R=0.000000,G=0.000000,B=0.000000,A=0.300000)" (+ (+ (Variables|Default|GetSize%20X) 1.0) -6e+01) (+ (+ (Variables|Default|GetSize%20Y) -1e+01) 0.0) 2.0 25.0)
          (HUD|DrawRect "(R=0.027451,G=0.913726,B=0.003922,A=0.301961)" (+ (+ (Variables|Default|GetSize%20X) -12.5) -6e+01) (+ (+ (Variables|Default|GetSize%20Y) 0.0) 0.0) 25.0 2.0)
          (HUD|DrawRect "(R=0.027451,G=0.913726,B=0.003922,A=0.301961)" (+ (+ (Variables|Default|GetSize%20X) -1.0) -6e+01) (+ (+ (Variables|Default|GetSize%20Y) -12.0) 0.0) 2.0 25.0)
          (HUD|DrawRect "(R=0.026241,G=0.913099,B=0.003677,A=1.000000)" (+ (+ (Variables|Default|GetSize%20X) -1.0) -6e+01) (+ (+ (Variables|Default|GetSize%20Y) 0.0) 0.0) 2.0 2.0)))
      (else
        ;[1 1 1] Crosshair (Ice Block)
        (if (== (Variables|/Game/Blueprints/BP_ThirdPersonCharacter.BP_ThirdPersonCharacter_C|GetAttackSelection _asbp_third_person_character) 1)
          (if (Variables|/Game/Blueprints/BP_ThirdPersonCharacter.BP_ThirdPersonCharacter_C|GetLeftShoulder? _asbp_third_person_character)
            (HUD|DrawRect "(R=0.000000,G=0.000000,B=0.000000,A=0.300000)" (+ (Variables|Default|GetSize%20X) 131.0) (+ (Variables|Default|GetSize%20Y) 51.0) 1e+02 2.0)
            (HUD|DrawRect "(R=0.000000,G=0.000000,B=1.000000,A=0.301961)" (+ (Variables|Default|GetSize%20X) 1.3e+02) (+ (Variables|Default|GetSize%20Y) 5e+01) 1e+02 2.0)
            (HUD|DrawRect "(R=0.000000,G=0.000000,B=1.000000,A=1.000000)" (+ (Variables|Default|GetSize%20X) 1.8e+02) (+ (Variables|Default|GetSize%20Y) 46.0) 4.0 4.0)
            (else
              (HUD|DrawRect "(R=0.000000,G=0.000000,B=0.000000,A=0.300000)" (+ (Variables|Default|GetSize%20X) -279.0) (+ (Variables|Default|GetSize%20Y) 51.0) 1e+02 2.0)
              (HUD|DrawRect "(R=0.000000,G=0.000000,B=1.000000,A=0.301961)" (+ (Variables|Default|GetSize%20X) -2.8e+02) (+ (Variables|Default|GetSize%20Y) 5e+01) 1e+02 2.0)
              (HUD|DrawRect "(R=0.000000,G=0.000000,B=1.000000,A=1.000000)" (+ (Variables|Default|GetSize%20X) -2.3e+02) (+ (Variables|Default|GetSize%20Y) 46.0) 4.0 4.0)))
          (else
            ;[1 1 1] Crosshair (Thunder Attack)
            (if (== (Variables|/Game/Blueprints/BP_ThirdPersonCharacter.BP_ThirdPersonCharacter_C|GetAttackSelection _asbp_third_person_character) 2)
              (if (Variables|/Game/Blueprints/BP_ThirdPersonCharacter.BP_ThirdPersonCharacter_C|GetLeftShoulder? _asbp_third_person_character)
                (HUD|DrawRect "(R=0.000000,G=0.000000,B=0.000000,A=0.300000)" (+ (+ (Variables|Default|GetSize%20X) -3.75) 4e+01) (+ (+ (Variables|Default|GetSize%20Y) 2.0) 0.0) 12.5 2.0)
                (HUD|DrawRect "(R=0.000000,G=0.000000,B=0.000000,A=0.300000)" (+ (+ (Variables|Default|GetSize%20X) 2.0) 4e+01) (+ (+ (Variables|Default|GetSize%20Y) -3.5) 0.0) 2.0 12.5)
                (HUD|DrawRect "(R=0.807843,G=0.721569,B=0.000000,A=0.301961)" (+ (+ (Variables|Default|GetSize%20X) -5.75) 4e+01) (+ (+ (Variables|Default|GetSize%20Y) 0.0) 0.0) 12.5 2.0)
                (HUD|DrawRect "(R=0.807843,G=0.721569,B=0.000000,A=0.301961)" (+ (+ (Variables|Default|GetSize%20X) 0.0) 4e+01) (+ (+ (Variables|Default|GetSize%20Y) -5.5) 0.0) 2.0 12.5)
                (HUD|DrawRect "(R=0.806952,G=0.723055,B=0.001518,A=1.000000)" (+ (+ (Variables|Default|GetSize%20X) 0.0) 4e+01) (+ (+ (Variables|Default|GetSize%20Y) 0.0) 0.0) 2.0 2.0)
                (else
                  (HUD|DrawRect "(R=0.000000,G=0.000000,B=0.000000,A=0.300000)" (+ (+ (Variables|Default|GetSize%20X) -3.75) -2e+01) (+ (+ (Variables|Default|GetSize%20Y) 2.0) 0.0) 12.5 2.0)
                  (HUD|DrawRect "(R=0.000000,G=0.000000,B=0.000000,A=0.300000)" (+ (+ (Variables|Default|GetSize%20X) 2.0) -2e+01) (+ (+ (Variables|Default|GetSize%20Y) -3.5) 0.0) 2.0 12.5)
                  (HUD|DrawRect "(R=0.807843,G=0.721569,B=0.000000,A=0.301961)" (+ (+ (Variables|Default|GetSize%20X) -5.75) -2e+01) (+ (+ (Variables|Default|GetSize%20Y) 0.0) 0.0) 12.5 2.0)
                  (HUD|DrawRect "(R=0.807843,G=0.721569,B=0.000000,A=0.301961)" (+ (+ (Variables|Default|GetSize%20X) 0.0) -2e+01) (+ (+ (Variables|Default|GetSize%20Y) -5.5) 0.0) 2.0 12.5)
                  (HUD|DrawRect "(R=0.806952,G=0.723055,B=0.001518,A=1.000000)" (+ (+ (Variables|Default|GetSize%20X) 0.0) -2e+01) (+ (+ (Variables|Default|GetSize%20Y) 0.0) 0.0) 2.0 2.0)))
              (elif (== (Variables|/Game/Blueprints/BP_ThirdPersonCharacter.BP_ThirdPersonCharacter_C|GetAttackSelection _asbp_third_person_character) 3)
                (if (Variables|/Game/Blueprints/BP_ThirdPersonCharacter.BP_ThirdPersonCharacter_C|GetLeftShoulder? _asbp_third_person_character)
                  ;[1 1 1] Crosshair (Fire Attack)
                  (HUD|DrawRect "(R=0.000000,G=0.000000,B=0.000000,A=0.300000)" (+ (+ (Variables|Default|GetSize%20X) -198.0) 2.6e+02) (+ (Variables|Default|GetSize%20Y) 2.0) 2.0 25.0)
                  (HUD|DrawRect "(R=0.000000,G=0.000000,B=0.000000,A=0.300000)" (+ (+ (Variables|Default|GetSize%20X) -88.0) 2.6e+02) (+ (Variables|Default|GetSize%20Y) 2.0) 2.0 25.0)
                  (HUD|DrawRect "(R=0.991102,G=0.000000,B=0.000000,A=0.300000)" (+ (+ (Variables|Default|GetSize%20X) -2e+02) 2.6e+02) (+ (Variables|Default|GetSize%20Y) 0.0) 2.0 25.0)
                  (HUD|DrawRect "(R=0.991102,G=0.000000,B=0.000000,A=0.300000)" (+ (+ (Variables|Default|GetSize%20X) -9e+01) 2.6e+02) (+ (Variables|Default|GetSize%20Y) 0.0) 2.0 25.0)
                  (HUD|DrawRect "(R=0.995000,G=0.000000,B=0.000000,A=1.000000)" (+ (+ (Variables|Default|GetSize%20X) -145.0) 2.6e+02) (+ (Variables|Default|GetSize%20Y) 12.0) 4.0 4.0)
                  (else
                    (HUD|DrawRect "(R=0.000000,G=0.000000,B=0.000000,A=0.300000)" (+ (Variables|Default|GetSize%20X) -198.0) (+ (Variables|Default|GetSize%20Y) 2.0) 2.0 25.0)
                    (HUD|DrawRect "(R=0.000000,G=0.000000,B=0.000000,A=0.300000)" (+ (Variables|Default|GetSize%20X) -88.0) (+ (Variables|Default|GetSize%20Y) 2.0) 2.0 25.0)
                    (HUD|DrawRect "(R=0.991102,G=0.000000,B=0.000000,A=0.300000)" (+ (Variables|Default|GetSize%20X) -2e+02) (+ (Variables|Default|GetSize%20Y) 0.0) 2.0 25.0)
                    (HUD|DrawRect "(R=0.991102,G=0.000000,B=0.000000,A=0.300000)" (+ (Variables|Default|GetSize%20X) -9e+01) (+ (Variables|Default|GetSize%20Y) 0.0) 2.0 25.0)
                    (HUD|DrawRect "(R=0.995000,G=0.000000,B=0.000000,A=1.000000)" (+ (Variables|Default|GetSize%20X) -145.0) (+ (Variables|Default|GetSize%20Y) 12.0) 4.0 4.0)))))))))
    (elif (== (Variables|/Game/Blueprints/BP_ThirdPersonCharacter.BP_ThirdPersonCharacter_C|GetAttackSelection _asbp_third_person_character) 1)
      (HUD|DrawText "(Q)      < 2. Ice Block >      (E)" "(R=0.000000,G=0.000000,B=0.000000,A=1.000000)" (+ (Variables|Default|GetSize%20X) -135.0) (+ (* SizeY 0.0) 30) 0 2.0 false)
      (HUD|DrawText "(Q)      < 2. Ice Block >      (E)" "(R=0.034340,G=0.356400,B=0.846873,A=1.000000)" (+ (Variables|Default|GetSize%20X) -137.0) (+ (* SizeY 0) 28) 0 2.0 false)
      (goto _label)
      (elif (== (Variables|/Game/Blueprints/BP_ThirdPersonCharacter.BP_ThirdPersonCharacter_C|GetAttackSelection _asbp_third_person_character) 2)
        (HUD|DrawText "(Q)    < 3. Thunderbolt >   (E)" "(R=0.000000,G=0.000000,B=0.000000,A=1.000000)" (+ (Variables|Default|GetSize%20X) -135.0) (+ (* SizeY 0.0) 30) 0 2.0 false)
        (HUD|DrawText "(Q)    < 3. Thunderbolt >   (E)" "(R=0.814847,G=0.737910,B=0.002125,A=1.000000)" (+ (Variables|Default|GetSize%20X) -137.0) (+ (* SizeY 0) 28) 0 2.0 false)
        (goto _label)
        (elif (== (Variables|/Game/Blueprints/BP_ThirdPersonCharacter.BP_ThirdPersonCharacter_C|GetAttackSelection _asbp_third_person_character) 3)
          (HUD|DrawText "(Q)  < 4. Flamethrower >  (E)" "(R=0.000000,G=0.000000,B=0.000000,A=1.000000)" (+ (Variables|Default|GetSize%20X) -135.0) (+ (* SizeY 0.0) 30) 0 2.0 false)
          (HUD|DrawText "(Q)  < 4. Flamethrower >  (E)" "(R=1.000000,G=0.278894,B=0.000000,A=1.000000)" (+ (Variables|Default|GetSize%20X) -137.0) (+ (* SizeY 0) 28) 0 2.0 false)
          (goto _label))))))

(fn ConstructionScript)