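; Ice block actor that encases a frozen enemy and melts after overlapping an actor tagged Hot.
; Once melting, each Tick shrinks the cube by Strength and refunds capped player Mana until it destroys itself.
; Tick also re-enables cube physics and sets enemy and helmet meshes from the player's FrozenEnemy index.
; It also destroys itself whenever the player's NewBlock equals the BlockType saved at BeginPlay, to replace old blocks.
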(event EventBeginPlay
  ;[1 1 1] Replace Block with New One
  (bind _asbp_third_person_character (Utilities|Casting|CastToBP_ThirdPersonCharacter (Game|GetPlayerCharacter 0)))
  (bind _output_get (Variables|Default|SetBlockType (Variables|/Game/Blueprints/BP_ThirdPersonCharacter.BP_ThirdPersonCharacter_C|GetNewBlock? _asbp_third_person_character))))

(event Collision|EventActorBeginOverlap
  (params (OtherActor :type Actor%20Object%20Reference))
  ;[1 1 1] Ice Hit with Fire
  (if (Actor|ActorHasTag OtherActor "Hot")
    (bind _output_get (Variables|Default|SetMelting? true))))

(event EventTick
  (params (DeltaSeconds :type Float%20%28single-precision%29))
  (bind _cube (Variables|Default|GetCube))
  (bind _helmet (Variables|Default|GetHelmet))
  (bind _frozenenemy (Variables|Default|GetFrozenEnemy))
  ;[1 1 1] Ice Hit with Fire
  (Physics|SetSimulatePhysics _cube true)
  (bind _asbp_third_person_character (Utilities|Casting|CastToBP_ThirdPersonCharacter (Game|GetPlayerCharacter 0)))
  ;[1 1 1] Replace Block with New One
  (if (== (Variables|/Game/Blueprints/BP_ThirdPersonCharacter.BP_ThirdPersonCharacter_C|GetNewBlock? (stale EventBeginPlay _asbp_third_person_character)) (stale EventBeginPlay _output_get))
    (Actor|DestroyActor)
    (elif (stale Collision|EventActorBeginOverlap _output_get)
      (if (<= (Variables|Default|GetStrength) 0.0)
        (Actor|DestroyActor)
        (else
          (Transformation|SetRelativeScale3D _cube (Math|Vector|MakeVector (Variables|Default|GetStrength) (Variables|Default|GetStrength) (Variables|Default|GetStrength)))
          (Variables|Default|SetStrength (- (Variables|Default|GetStrength) 0.125))
          (Variables|/Game/Blueprints/BP_ThirdPersonCharacter.BP_ThirdPersonCharacter_C|SetMana _asbp_third_person_character (+ (Variables|/Game/Blueprints/BP_ThirdPersonCharacter.BP_ThirdPersonCharacter_C|GetMana _asbp_third_person_character) 1.0))
          (if (> (Variables|/Game/Blueprints/BP_ThirdPersonCharacter.BP_ThirdPersonCharacter_C|GetMana _asbp_third_person_character) 1e+02)
            (Variables|/Game/Blueprints/BP_ThirdPersonCharacter.BP_ThirdPersonCharacter_C|SetMana _asbp_third_person_character 1e+02))
          ;[1 1 1] Frozen Enemy
          (if (== (Variables|/Game/Blueprints/BP_ThirdPersonCharacter.BP_ThirdPersonCharacter_C|GetFrozenEnemy _asbp_third_person_character) 0) :!label _label
            (Class|SkinnedMeshComponent|SetSkeletalMesh _frozenenemy 0 true)
            (Components|StaticMesh|SetStaticMesh _helmet 0)
            (elif (== (Variables|/Game/Blueprints/BP_ThirdPersonCharacter.BP_ThirdPersonCharacter_C|GetFrozenEnemy _asbp_third_person_character) 1)
              (Class|SkinnedMeshComponent|SetSkeletalMesh _frozenenemy "/Game/Assets/CityofBrass_Enemies/Meshes/Enemy/Large/Large_Mesh.Large_Mesh" true)
              (Components|StaticMesh|SetStaticMesh _helmet 0)
              (elif (== (Variables|/Game/Blueprints/BP_ThirdPersonCharacter.BP_ThirdPersonCharacter_C|GetFrozenEnemy _asbp_third_person_character) 2)
                (Class|SkinnedMeshComponent|SetSkeletalMesh _frozenenemy "/Game/Assets/CityofBrass_Enemies/Meshes/Enemy/Charger/Charger.Charger" true)
                (Components|StaticMesh|SetStaticMesh _helmet "/Game/Assets/CityofBrass_Enemies/Meshes/Enemy/Charger/Charger_Helmet.Charger_Helmet")
                (elif (== (Variables|/Game/Blueprints/BP_ThirdPersonCharacter.BP_ThirdPersonCharacter_C|GetFrozenEnemy _asbp_third_person_character) 3)
                  (Class|SkinnedMeshComponent|SetSkeletalMesh _frozenenemy "/Game/Assets/CityofBrass_Enemies/Meshes/Enemy/Wizard/Wizard_Mesh.Wizard_Mesh" true)
                  (Components|StaticMesh|SetStaticMesh _helmet 0)))))))
      (else
        (goto _label)))))

(fn ConstructionScript)