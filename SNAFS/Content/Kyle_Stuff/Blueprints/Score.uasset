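; Score is a pickup Actor that awards the player 50 points when touched.
; Tick accumulates time and sets the actor's world Z from a sine wave, so it bobs around a fixed height regardless of where it is placed.
; On overlap, it checks that the other actor's first tag is Player, casts to Player_Character, calls AddPoints and destroys itself.
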(event Collision|EventActorBeginOverlap
  (params (OtherActor :type Actor%20Object%20Reference))
  (bind _tags (Variables|/Script/Engine.Actor|GetTags OtherActor))
  (if (> (Utilities|Array|Length _tags) 0)
    (if (== (Utilities|Array|Get(acopy) _tags) "Player")
      (bind _asplayer_character (Utilities|Casting|CastToPlayer_Character OtherActor))
      (Default|AddPoints _asplayer_character 50)
      (Actor|DestroyActor))))

(event EventTick
  (params (DeltaSeconds :type Float%20%28single-precision%29))
  (bind _returnvalue (Transformation|GetActorLocation))
  (Variables|Default|SetTimer (+ DeltaSeconds (Variables|Default|GetTimer)))
  (Transformation|SetActorLocation (Math|Vector|MakeVector (.x _returnvalue) (.y _returnvalue) (+ (* (Math|Trig|Sin(Radians) (* (Variables|Default|GetTimer) 2.5)) 3e+01) 1e+02)) false false))

(fn ConstructionScript)