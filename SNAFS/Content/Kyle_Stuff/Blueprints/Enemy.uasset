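; Enemy that walks toward the player's last seen location, damaging and knocking back the player on contact.
; Pawn Sensing updates the target while Tick turns and sweeps it forward, with a walk cycle faked by timed static mesh swaps.
; Bullet overlaps apply damage and an impulse scaled by bullet speed, flashing materials; IFrames throttles only the flash.
; At zero health it awards the player points and destroys itself.
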(event OnSeePawn(PawnSensing)
  (params (Pawn :type Pawn%20Object%20Reference))
  (bind _returnvalue (Game|GetPlayerCharacter 0))
  (if (== Pawn _returnvalue)
    (Variables|Default|SetTarget (Transformation|GetActorLocation _returnvalue))))

(event OnComponentBeginOverlap(Hurtbox)
  (params (OverlappedComponent :type Primitive%20Component%20Object%20Reference) (OtherActor :type Actor%20Object%20Reference) (OtherComp :type Primitive%20Component%20Object%20Reference) (OtherBodyIndex :type Integer) (bFromSweep :type Boolean) (SweepResult :type Hit%20Result%20Structure%20%28by%20ref%29))
  (bind _returnvalue (Transformation|GetVelocity OtherActor))
  (bind _tags (Variables|/Script/Engine.Actor|GetTags OtherActor))
  (bind _returnvalue_2 (Math|Vector|VectorLength _returnvalue))
  (if (> (Utilities|Array|Length _tags) 0)
    (if (== (Utilities|Array|Get(acopy) _tags) "Bullet")
      (Physics|AddImpulse (Variables|Character|GetCharacterMovement) (* (Math|Vector|GetForwardVector (Transformation|GetActorRotation)) (* _returnvalue_2 (Variables|Default|GetDamageForce))) true)
      (CallFunction|TakeDamageEnemy "/Game/Jade_Stuff/Textures/MAT_Villain.MAT_Villain" (* (Variables|Default|GetDamageMult) _returnvalue_2)))))

(event Custom|Take%20Damage%20Enemy
  (params (Material :type Material%20Interface%20Object%20Reference) (Force :type Float%20%28double-precision%29))
  (Audio|PlaySound2D "/Game/Jamal_Stuff/Hit.Hit" 1.0 1.0 0.0 0 0)
  (bind _output_get (Variables|Default|SetHealth (- (Variables|Default|GetHealth) Force)))
  (if (<= _output_get 0.0)
    (bind _asplayer_character (Utilities|Casting|CastToPlayer_Character (Game|GetPlayerCharacter 0)))
    (Default|AddPoints _asplayer_character 100)
    (Actor|DestroyActor)
    (elif (not (Variables|Default|GetDamaged))
      (Rendering|Material|SetMaterial (Variables|Default|GetHat) 0 "/Engine/VREditor/BasicMeshes/MI_Cube_01.MI_Cube_01")
      (Rendering|Material|SetMaterial (Variables|Character|GetMesh) 0 "/Engine/VREditor/BasicMeshes/MI_Cube_01.MI_Cube_01")
      (Utilities|FlowControl|Sequence
        (:then_0
          (Utilities|FlowControl|Delay 0.2)
          (Rendering|Material|SetMaterial (Variables|Character|GetMesh) 0 Material)
          (Rendering|Material|SetMaterial (Variables|Default|GetHat) 0 "/Game/Kyle_Stuff/Materials/MAT_Villain_Hat.MAT_Villain_Hat"))
        (:then_1
          (Variables|Default|SetDamaged true)
          (Utilities|FlowControl|Delay (Variables|Default|GetIFrames))
          (Variables|Default|SetDamaged false))))))

(event Custom|Animation
  (bind _body (Variables|Default|GetBody))
  (bind _walk_speed (Variables|Default|GetWalk%20Speed))
  (if (and (Utilities|Operators|NotEqual(!=) (Transformation|GetActorLocation) (Variables|Default|GetTarget) 25.0) (not (Variables|Default|GetAnimating)))
    (Variables|Default|SetAnimating true)
    (Components|StaticMesh|SetStaticMesh _body "/Game/Jade_Stuff/Anim_stuff/Elton_Bat_Left.Elton_Bat_Left")
    (Utilities|FlowControl|Delay _walk_speed)
    (Components|StaticMesh|SetStaticMesh _body "/Game/Jade_Stuff/Animation/Elton_Bat_Idle_New.Elton_Bat_Idle_New")
    (Utilities|FlowControl|Delay _walk_speed)
    (Components|StaticMesh|SetStaticMesh _body "/Game/Jade_Stuff/Animation/Elton_Bat_Right.Elton_Bat_Right")
    (Utilities|FlowControl|Delay _walk_speed)
    (Components|StaticMesh|SetStaticMesh _body "/Game/Jade_Stuff/Animation/Elton_Bat_Idle_New.Elton_Bat_Idle_New")
    (Utilities|FlowControl|Delay _walk_speed)
    (Variables|Default|SetAnimating false)))

(event EventBeginPlay
  (Variables|Default|SetTarget (Transformation|GetActorLocation)))

(event Collision|EventHit
  (params (MyComp :type Primitive%20Component%20Object%20Reference) (Other :type Actor%20Object%20Reference) (OtherComp :type Primitive%20Component%20Object%20Reference) (bSelfMoved :type Boolean) (HitLocation :type Vector :default "0, 0, 0") (HitNormal :type Vector :default "0, 0, 0") (NormalImpulse :type Vector :default "0, 0, 0") (Hit :type Hit%20Result%20Structure%20%28by%20ref%29))
  (bind _tags (Variables|/Script/Engine.Actor|GetTags Other))
  (if (> (Utilities|Array|Length _tags) 0)
    (if (== (Utilities|Array|Get(acopy) _tags) "Player")
      (bind _asplayer_character (Utilities|Casting|CastToPlayer_Character Other))
      (Default|TakeDamage _asplayer_character "/Game/Jade_Stuff/Textures/MAT_Elton.MAT_Elton")
      (Physics|AddImpulse (Variables|/Script/Engine.Character|GetCharacterMovement _asplayer_character) (* HitNormal (Variables|Default|GetHitForce)) true))))

(event EventTick
  (params (DeltaSeconds :type Float%20%28single-precision%29))
  (bind _returnvalue (Transformation|GetActorTransform))
  (bind _returnvalue_2 (Transformation|GetActorLocation))
  (bind _target (Variables|Default|GetTarget))
  (CallFunction|Animation)
  (if (Utilities|Operators|NotEqual(!=) _returnvalue_2 _target 25.0)
    (Transformation|SetActorRotation (Math|Rotator|MakeRotator (.roll (.rotation _returnvalue)) (.pitch (.rotation _returnvalue)) (.yaw (Math|Rotator|FindLookatRotation _returnvalue_2 _target))))
    (Transformation|SetActorLocation (+ _returnvalue_2 (* (Math|Vector|GetForwardVector (Transformation|GetActorRotation)) (* DeltaSeconds (Variables|Default|GetSpeed)))) true false)))

(fn ConstructionScript)