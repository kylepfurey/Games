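; Random_Seed sets up a shared random stream and seed when play begins and passes both out through StartEvents.
; MakeRandomStream gets a seed from GetRandomSeed using the randomize toggle and min/max settings, applies it to the stream and prints it on screen.
; GetRandomStream and GetSeed are identical getters returning both values.
; GetRandomSeed's random-or-current selection logic appears unconnected.
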(event EventBeginPlay
  ;[0 1 0.2706] Initializes the random stream with the seed and calls the start events with the new seed
  (bind (_random_stream _seed) (CallFunction|MakeRandomStream))
  (Default|CallStartEvents _random_stream _seed))

(fn ConstructionScript)

(fn MakeRandomStream
  ;[0 1 0.2706] Makes the random stream with a random seed based on the random seed settings
  (bind _output_get (Variables|Default|SetSeed (Utilities|GetRandomSeed (Variables|Default|GetSeed) (Variables|Default|GetRandomize%20Seed) (Variables|Default|GetSeed%20Minimum) (Variables|Default|GetSeed%20Maximum))))
  (Math|Random|SetRandomStreamSeed (Variables|Default|GetRandom%20Stream) _output_get)
  (Development|PrintString (Utilities|String|Append "New Seed: " (Utilities|String|ToString(Integer) _output_get)) true true "(R=0.000000,G=1.000000,B=0.270588,A=1.000000)" 3.0 "Seed")
  (return (Variables|Default|GetRandom%20Stream) (Variables|Default|GetSeed)))

(fn GetRandomStream
  ;[0 1 0.2706] Returns the random stream and seed
  (return (Variables|Default|GetRandom%20Stream) (Variables|Default|GetSeed)))

(fn GetSeed
  ;[0 1 0.2706] Returns the random stream and seed
  (return (Variables|Default|GetRandom%20Stream) (Variables|Default|GetSeed)))