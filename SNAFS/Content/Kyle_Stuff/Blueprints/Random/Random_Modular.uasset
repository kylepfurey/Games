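; Random modular spawner that populates named sets of spawn points with module actors picked by weighted chance from a random stream.
; Spawn builds a table from each set's allowed modules, then fills points in order, applying offsets and optional transform randomization.
; Spawn-count caps and exclusivity modifiers that push a rate to zero remove modules from the table.
; Spawned actors are tracked per set for despawning before respawns.
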(fn ConstructionScript)

(fn SpawnSet
  (params (Set%20Name :type Name))
  ;[0.1928 0 1] Spawn modules for a specific set
  (CallFunction|DespawnSet Set%20Name)
  (for _array_element (Variables|Default|GetSets)
    (if (== Set%20Name (Utilities|Struct|BreakSet_Of_Modules _array_element))
      (CallFunction|Spawn _array_element)
      (return))))

(fn SpawnAll
  ;[0.1928 0 1] Spawn modules for all sets
  (CallFunction|DespawnAll)
  (for _array_element (Variables|Default|GetSets)
    (CallFunction|Spawn _array_element)))

(fn DespawnSet
  (params (Set%20Name :type Name))
  ;[0.1928 0 1] Destroys all spawned modules of a given set
  (for _array_element (Variables|Default|GetSets)
    (if (== Set%20Name (Utilities|Struct|BreakSet_Of_Modules _array_element))
      (for _array_element_2 (Utilities|Struct|BreakSpawned_Actors (.Value (Utilities|Map|Find (Variables|Default|GetAll%20Spawned%20Modules) (Utilities|Struct|BreakSet_Of_Modules _array_element))))
        (Actor|DestroyActor))
      (Utilities|Map|Remove (Variables|Default|GetAll%20Spawned%20Modules) (Utilities|Struct|BreakSet_Of_Modules _array_element))
      (return))))

(fn DespawnAll
  (bind _all_spawned_modules (Variables|Default|GetAll%20Spawned%20Modules))
  ;[0.1928 0 1] Destroys all spawned modules of each set
  (for _array_element (Variables|Default|GetSets)
    (if (Utilities|Map|Contains (Variables|Default|GetAll%20Spawned%20Modules) (Utilities|Struct|BreakSet_Of_Modules _array_element))
      (for _array_element_2 (Utilities|Struct|BreakSpawned_Actors (.Value (Utilities|Map|Find _all_spawned_modules (Utilities|Struct|BreakSet_Of_Modules _array_element))))
        (Actor|DestroyActor _array_element_2))))
  (Utilities|Map|Clear _all_spawned_modules))

(fn Spawn
  (params (Set :type Set%20Of%20Modules%20Structure))
  (bind _all_modules (Variables|Default|GetAll%20Modules))
  (bind _random_stream (Variables|Default|GetRandom%20Stream))
  (bind _all_spawned_modules (Variables|Default|GetAll%20Spawned%20Modules))
  ;[0.1928 0 1] Spawns modules at random depending on their spawn rates from a given set
  (if (.useallmodules Set)
    (for _array_element _all_modules
      (Utilities|Array|Add (LocalVariables|GetSpawn%20Table) _array_element)
      (Utilities|Map|Add (LocalVariables|GetSpawn%20Rates) (.Name (Utilities|Struct|BreakModule _array_element)) (.SpawnRate (Utilities|Struct|BreakModule _array_element))))
    (else
      (for _array_element_2 _all_modules
        (if (Utilities|Array|ContainsItem (.setmodules Set) (.Name (Utilities|Struct|BreakModule _array_element_2)))
          (Utilities|Array|Add (LocalVariables|GetSpawn%20Table) _array_element_2)
          (Utilities|Map|Add (LocalVariables|GetSpawn%20Rates) (.Name (Utilities|Struct|BreakModule _array_element_2)) (.SpawnRate (Utilities|Struct|BreakModule _array_element_2)))))))
  (for _array_element_3 (.spawnpoints Set)
    (Utilities|Array|Add (LocalVariables|GetSpawn%20Points) _array_element_3))
  (while (and (> (Utilities|Array|Length (LocalVariables|GetSpawn%20Table)) 0) (> (Utilities|Array|Length (LocalVariables|GetSpawn%20Points)) 0))
    (LocalVariables|SetSpawn%20Percent 0.0)
    (Utilities|Map|Clear (LocalVariables|GetSpawn%20Percents))
    (for _array_element_4 (LocalVariables|GetSpawn%20Table)
      (if (or (<= (.Value (Utilities|Map|Find (LocalVariables|GetSpawn%20Rates) (.Name (Utilities|Struct|BreakModule _array_element_4)))) 0.0) (<= (.NumberOfSpawns (Utilities|Struct|BreakModule _array_element_4)) (CallFunction|FindAll (LocalVariables|GetSpawned%20Modules) _array_element_4)))
        (Utilities|Array|RemoveItem (LocalVariables|GetSpawn%20Table) _array_element_4)
        (else
          (bind _output_get (LocalVariables|SetSpawn%20Percent (+ (.SpawnRate (Utilities|Struct|BreakModule _array_element_4)) (LocalVariables|GetSpawn%20Percent))))
          (Utilities|Map|Add (LocalVariables|GetSpawn%20Percents) (.Name (Utilities|Struct|BreakModule _array_element_4)) _output_get))))
    (LocalVariables|SetSpawn%20Percent (Math|Random|RandomFloatinRangefromStream (Variables|Default|GetRandom%20Stream) 0.0 (LocalVariables|GetSpawn%20Percent)))
    (bind _keys (Utilities|Map|Keys (LocalVariables|GetSpawn%20Percents)))
    (LocalVariables|SetBREAK false)
    (bind _array_element_5 (Utilities|Array|ForEachLoopwithBreak _keys :!label _label)
      (:LoopBody
        (if (not (LocalVariables|GetBREAK))
          (if (< (LocalVariables|GetSpawn%20Percent) (.Value (Utilities|Map|Find (LocalVariables|GetSpawn%20Percents) _array_element_5)))
            (LocalVariables|SetSpawn%20Point (Utilities|Array|Get(acopy) (LocalVariables|GetSpawn%20Points)))
            (Utilities|Array|RemoveIndex (LocalVariables|GetSpawn%20Points))
            (bind _module_data (Utilities|GetModuleDatafromName _array_element_5)
              (:__
                (bind _returnvalue (Game|SpawnActorfromClass (.ActorClass (Utilities|Struct|BreakModule _module_data)) (Math|Transform|MakeTransform (+ (.SpawnPositionOffset (Utilities|Struct|BreakModule _module_data)) (.location (Transformation|GetActorTransform (LocalVariables|GetSpawn%20Point)))) (Math|Rotator|CombineRotators (.SpawnRotationOffset (Utilities|Struct|BreakModule _module_data)) (.rotation (Transformation|GetActorTransform (LocalVariables|GetSpawn%20Point)))) (.SpawnScale (Utilities|Struct|BreakModule _module_data))) "AdjustIfPossibleButAlwaysSpawn" "MultiplyWithRoot" 0 0))
                (bind _output_get_2 (LocalVariables|SetSpawned%20Module _returnvalue))
                (if (.RandomizeTransform (Utilities|Struct|BreakModule _module_data))
                  (Transformation|SetActorTransform (LocalVariables|GetSpawned%20Module) (Math|Transform|MakeTransform (+ (.location (Transformation|GetActorTransform _output_get_2)) (Math|Vector|MakeVector (.New%20Float%20X (Utilities|RandomizeThreeFloats _random_stream (.x (Utilities|Array|Get(acopy) (.RandomSpawnPositionOffsetRange (Utilities|Struct|BreakModule _module_data)))) (.x (Utilities|Array|Get(acopy) (.RandomSpawnPositionOffsetRange (Utilities|Struct|BreakModule _module_data)) 1)) (.y (Utilities|Array|Get(acopy) (.RandomSpawnPositionOffsetRange (Utilities|Struct|BreakModule _module_data)))) (.y (Utilities|Array|Get(acopy) (.RandomSpawnPositionOffsetRange (Utilities|Struct|BreakModule _module_data)) 1)) (.z (Utilities|Array|Get(acopy) (.RandomSpawnPositionOffsetRange (Utilities|Struct|BreakModule _module_data)))) (.z (Utilities|Array|Get(acopy) (.RandomSpawnPositionOffsetRange (Utilities|Struct|BreakModule _module_data)) 1)))) (.New%20Float%20Y (Utilities|RandomizeThreeFloats _random_stream (.x (Utilities|Array|Get(acopy) (.RandomSpawnPositionOffsetRange (Utilities|Struct|BreakModule _module_data)))) (.x (Utilities|Array|Get(acopy) (.RandomSpawnPositionOffsetRange (Utilities|Struct|BreakModule _module_data)) 1)) (.y (Utilities|Array|Get(acopy) (.RandomSpawnPositionOffsetRange (Utilities|Struct|BreakModule _module_data)))) (.y (Utilities|Array|Get(acopy) (.RandomSpawnPositionOffsetRange (Utilities|Struct|BreakModule _module_data)) 1)) (.z (Utilities|Array|Get(acopy) (.RandomSpawnPositionOffsetRange (Utilities|Struct|BreakModule _module_data)))) (.z (Utilities|Array|Get(acopy) (.RandomSpawnPositionOffsetRange (Utilities|Struct|BreakModule _module_data)) 1)))) (.New%20Float%20Z (Utilities|RandomizeThreeFloats _random_stream (.x (Utilities|Array|Get(acopy) (.RandomSpawnPositionOffsetRange (Utilities|Struct|BreakModule _module_data)))) (.x (Utilities|Array|Get(acopy) (.RandomSpawnPositionOffsetRange (Utilities|Struct|BreakModule _module_data)) 1)) (.y (Utilities|Array|Get(acopy) (.RandomSpawnPositionOffsetRange (Utilities|Struct|BreakModule _module_data)))) (.y (Utilities|Array|Get(acopy) (.RandomSpawnPositionOffsetRange (Utilities|Struct|BreakModule _module_data)) 1)) (.z (Utilities|Array|Get(acopy) (.RandomSpawnPositionOffsetRange (Utilities|Struct|BreakModule _module_data)))) (.z (Utilities|Array|Get(acopy) (.RandomSpawnPositionOffsetRange (Utilities|Struct|BreakModule _module_data)) 1)))))) (Math|Rotator|CombineRotators (.rotation (Transformation|GetActorTransform _output_get_2)) (Math|Rotator|MakeRotator (.New%20Float%20X (Utilities|RandomizeThreeFloats _random_stream (.roll (Utilities|Array|Get(acopy) (.RandomSpawnRotationOffsetRange (Utilities|Struct|BreakModule _module_data)))) (.roll (Utilities|Array|Get(acopy) (.RandomSpawnRotationOffsetRange (Utilities|Struct|BreakModule _module_data)) 1)) (.pitch (Utilities|Array|Get(acopy) (.RandomSpawnRotationOffsetRange (Utilities|Struct|BreakModule _module_data)))) (.pitch (Utilities|Array|Get(acopy) (.RandomSpawnRotationOffsetRange (Utilities|Struct|BreakModule _module_data)) 1)) (.yaw (Utilities|Array|Get(acopy) (.RandomSpawnRotationOffsetRange (Utilities|Struct|BreakModule _module_data)))) (.yaw (Utilities|Array|Get(acopy) (.RandomSpawnRotationOffsetRange (Utilities|Struct|BreakModule _module_data)) 1)))) (.New%20Float%20Y (Utilities|RandomizeThreeFloats _random_stream (.roll (Utilities|Array|Get(acopy) (.RandomSpawnRotationOffsetRange (Utilities|Struct|BreakModule _module_data)))) (.roll (Utilities|Array|Get(acopy) (.RandomSpawnRotationOffsetRange (Utilities|Struct|BreakModule _module_data)) 1)) (.pitch (Utilities|Array|Get(acopy) (.RandomSpawnRotationOffsetRange (Utilities|Struct|BreakModule _module_data)))) (.pitch (Utilities|Array|Get(acopy) (.RandomSpawnRotationOffsetRange (Utilities|Struct|BreakModule _module_data)) 1)) (.yaw (Utilities|Array|Get(acopy) (.RandomSpawnRotationOffsetRange (Utilities|Struct|BreakModule _module_data)))) (.yaw (Utilities|Array|Get(acopy) (.RandomSpawnRotationOffsetRange (Utilities|Struct|BreakModule _module_data)) 1)))) (.New%20Float%20Z (Utilities|RandomizeThreeFloats _random_stream (.roll (Utilities|Array|Get(acopy) (.RandomSpawnRotationOffsetRange (Utilities|Struct|BreakModule _module_data)))) (.roll (Utilities|Array|Get(acopy) (.RandomSpawnRotationOffsetRange (Utilities|Struct|BreakModule _module_data)) 1)) (.pitch (Utilities|Array|Get(acopy) (.RandomSpawnRotationOffsetRange (Utilities|Struct|BreakModule _module_data)))) (.pitch (Utilities|Array|Get(acopy) (.RandomSpawnRotationOffsetRange (Utilities|Struct|BreakModule _module_data)) 1)) (.yaw (Utilities|Array|Get(acopy) (.RandomSpawnRotationOffsetRange (Utilities|Struct|BreakModule _module_data)))) (.yaw (Utilities|Array|Get(acopy) (.RandomSpawnRotationOffsetRange (Utilities|Struct|BreakModule _module_data)) 1)))))) (+ (.scale (Transformation|GetActorTransform _output_get_2)) (Math|Vector|MakeVector (.New%20Float%20X (Utilities|RandomizeThreeFloats _random_stream (.x (Utilities|Array|Get(acopy) (.RandomSpawnScaleRange (Utilities|Struct|BreakModule _module_data)))) (.x (Utilities|Array|Get(acopy) (.RandomSpawnScaleRange (Utilities|Struct|BreakModule _module_data)) 1)) (.y (Utilities|Array|Get(acopy) (.RandomSpawnScaleRange (Utilities|Struct|BreakModule _module_data)))) (.y (Utilities|Array|Get(acopy) (.RandomSpawnScaleRange (Utilities|Struct|BreakModule _module_data)) 1)) (.z (Utilities|Array|Get(acopy) (.RandomSpawnScaleRange (Utilities|Struct|BreakModule _module_data)))) (.z (Utilities|Array|Get(acopy) (.RandomSpawnScaleRange (Utilities|Struct|BreakModule _module_data)) 1)))) (.New%20Float%20Y (Utilities|RandomizeThreeFloats _random_stream (.x (Utilities|Array|Get(acopy) (.RandomSpawnScaleRange (Utilities|Struct|BreakModule _module_data)))) (.x (Utilities|Array|Get(acopy) (.RandomSpawnScaleRange (Utilities|Struct|BreakModule _module_data)) 1)) (.y (Utilities|Array|Get(acopy) (.RandomSpawnScaleRange (Utilities|Struct|BreakModule _module_data)))) (.y (Utilities|Array|Get(acopy) (.RandomSpawnScaleRange (Utilities|Struct|BreakModule _module_data)) 1)) (.z (Utilities|Array|Get(acopy) (.RandomSpawnScaleRange (Utilities|Struct|BreakModule _module_data)))) (.z (Utilities|Array|Get(acopy) (.RandomSpawnScaleRange (Utilities|Struct|BreakModule _module_data)) 1)))) (.New%20Float%20Z (Utilities|RandomizeThreeFloats _random_stream (.x (Utilities|Array|Get(acopy) (.RandomSpawnScaleRange (Utilities|Struct|BreakModule _module_data)))) (.x (Utilities|Array|Get(acopy) (.RandomSpawnScaleRange (Utilities|Struct|BreakModule _module_data)) 1)) (.y (Utilities|Array|Get(acopy) (.RandomSpawnScaleRange (Utilities|Struct|BreakModule _module_data)))) (.y (Utilities|Array|Get(acopy) (.RandomSpawnScaleRange (Utilities|Struct|BreakModule _module_data)) 1)) (.z (Utilities|Array|Get(acopy) (.RandomSpawnScaleRange (Utilities|Struct|BreakModule _module_data)))) (.z (Utilities|Array|Get(acopy) (.RandomSpawnScaleRange (Utilities|Struct|BreakModule _module_data)) 1)))))))))
                (Utilities|Array|Add (LocalVariables|GetSpawned%20Modules) _module_data)
                (bind _output_get_3 (LocalVariables|SetSpawned%20Actors%20Copy (.Value (Utilities|Map|Find _all_spawned_modules (.name Set)))))
                (Utilities|Array|Add (.spawnedactors _output_get_3) (LocalVariables|GetSpawned%20Module))
                (Utilities|Map|Add _all_spawned_modules (.name Set) (LocalVariables|GetSpawned%20Actors%20Copy))
                (for _array_element_6 (LocalVariables|GetSpawn%20Table)
                  (LocalVariables|SetBREAK2 false)
                  (bind _array_element_7 (Utilities|Array|ForEachLoopwithBreak (.ExclusiveModules (Utilities|Struct|BreakModule _array_element_6)) :!label _label_2)
                    (:LoopBody
                      (if (not (LocalVariables|GetBREAK2))
                        (if (== _array_element_5 (.ExclusiveModuleName (Utilities|Struct|BreakExclusive_Module _array_element_7)))
                          (Utilities|Map|Add (LocalVariables|GetSpawn%20Rates) (.Name (Utilities|Struct|BreakModule _array_element_6)) (+ (.Value (Utilities|Map|Find (LocalVariables|GetSpawn%20Rates) (.Name (Utilities|Struct|BreakModule _array_element_6)))) (.SpawnModifier (Utilities|Struct|BreakExclusive_Module _array_element_7))))
                          (LocalVariables|SetBREAK2 true)
                          (goto _label_2 Break))))))
                (Rendering|SetActorHiddenInGame (LocalVariables|GetSpawn%20Point) true)
                (LocalVariables|SetBREAK true)
                (goto _label Break)))))))))

(fn FindAll
  (params (Array :type Array%20of%20Module%20Structures) (Element :type Module%20Structure))
  ;[0.1928 0 1] Returns a count of specific elements in an array
  (for _array_element Array
    (if (== (Utilities|Struct|BreakModule _array_element) (Utilities|Struct|BreakModule Element))
      (Math|Integer|IncrementInt (LocalVariables|GetCount))))
  (return (LocalVariables|GetCount)))

(fn TestSpawn
  ;[0.1928 0 1] Test spawning when in play mode
  (if (Utilities|IsValid (Game|GetGameInstance))
    (CallFunction|SpawnAll)
    (else
      (Development|PrintString "No spawning unless in play mode!" true true "(R=1.000000,G=0.088576,B=0.000000,A=1.000000)" 2.0 "No Spawning"))))