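; Game manager that runs rounds of a spotlight posing game, tracking difficulty, quota, cumulative points and high score.
; GameStart sets the player's timer, raises the quota and shrinks the spotlight.
; GameEnd scores spotlight and player distance from targets plus pose and mask matches, then reloads Game on a win or resets to MainMenu on a loss.
; Wins can raise difficulty, which makes SetTarget randomise pose, then also mask.
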(event Custom|Win
  (params (Points :type Float%20%28double-precision%29))
  ;[1 1 1] Game loop
  (bind _output_get (Variables|Default|SetSpotLightSize (- (stale _output_get) (Variables|Default|GetSpotLightSizeDecrease))))
  (bind _output_get_2 (Variables|Default|SetDisplayedPoints (+ Points (Variables|Default|GetDisplayedPoints))))
  (CallFunction|HighScore _output_get_2)
  (if (and (>= _output_get_2 (Variables|Default|GetHardThreshold)) (Utilities|Enum|Equal(Enum) (Variables|Default|GetDifficulty) "NewEnumerator1"))
    (Variables|Default|SetDifficulty "NewEnumerator2")
    (elif (and (>= _output_get_2 (Variables|Default|GetMediumThreshold)) (Utilities|Enum|Equal(Enum) (Variables|Default|GetDifficulty) "NewEnumerator0"))
      (Variables|Default|SetDifficulty "NewEnumerator1")))
  (Game|OpenLevel(byObjectReference) "/Game/KyleStuff/Levels/Game.Game"))

(event Custom|Lose
  (params (Points :type Float%20%28double-precision%29))
  (bind (_difficulty _targetmaxdistance _targetpose _posepoints _targetmask _maskpoints _spotlightsize _spotlightminsize _spotlightsizedecrease _displayedpoints _highestpoints _maxpoints _hardthreshold _mediumthreshold _quota) (Utilities|GetClassDefaults "GameManager_C"))
  ;[1 1 1] Game loop
  (CallFunction|HighScore (+ Points (Variables|Default|GetDisplayedPoints)))
  (Variables|Default|SetSpotLightSize _spotlightsize)
  (Variables|Default|SetDisplayedPoints _displayedpoints)
  (Variables|Default|SetQuota _quota)
  (Game|OpenLevel(byObjectReference) "/Game/KyleStuff/Levels/MainMenu.MainMenu"))

(event Custom|GameEnd
  ;[1 1 1] Game loop
  (bind _asplayer (Utilities|Casting|CastToPlayer (Game|GetPlayerCharacter 0)))
  (Variables|/Game/KyleStuff/Player/Player.Player_C|SetCanMove _asplayer false)
  (Variables|/Game/KyleStuff/Player/Player.Player_C|SetControlSpotLight _asplayer false)
  (bind _totaldifference (CallFunction|DifferenceCalculator))
  (bind _points (CallFunction|PointCalculator _totaldifference (Utilities|Enum|Equal(Enum) (Variables|Default|GetTargetPose) (Variables|/Game/KyleStuff/Player/Player.Player_C|GetCurrentPose _asplayer)) (Utilities|Enum|Equal(Enum) (Variables|Default|GetTargetMask) (Variables|/Game/KyleStuff/Player/Player.Player_C|GetCurrentMask _asplayer))))
  (bind _output_get (Variables|/Game/KyleStuff/Player/Player.Player_C|SetPoints _asplayer (+ _points (Variables|Default|GetDisplayedPoints))))
  (Utilities|FlowControl|Delay 7.5)
  (if (>= _output_get (Variables|Default|GetQuota))
    (CallFunction|Win _points)
    (else
      (CallFunction|Lose _points))))

(event Custom|GameStart
  (bind _spotlightminsize (Variables|Default|GetSpotLightMinSize))
  ;[1 1 1] Game loop
  (bind _asplayer (Utilities|Casting|CastToPlayer (Game|GetPlayerCharacter 0)))
  (Variables|/Game/KyleStuff/Player/Player.Player_C|SetTimer _asplayer (Utilities|Select :Index (Variables|Default|GetDifficulty) :NewEnumerator0 2e+01 :NewEnumerator1 15.0 :NewEnumerator2 15.0))
  (Variables|Default|SetQuota (+ (Variables|Default|GetQuota) (Utilities|Select :Index (Variables|Default|GetDifficulty) :NewEnumerator0 2e+02 :NewEnumerator1 5e+02 :NewEnumerator2 8e+02)))
  (Variables|Default|SetSpotLightSize (- (Variables|Default|GetSpotLightSize) (Variables|Default|GetSpotLightSizeDecrease)))
  (if (< (Variables|Default|GetSpotLightSize) _spotlightminsize)
    (Variables|Default|SetSpotLightSize _spotlightminsize))
  (bind _asplayer_2 (Utilities|Casting|CastToPlayer (Game|GetPlayerCharacter 0)))
  (Variables|/Game/KyleStuff/Player/Player.Player_C|SetSpotLightSize _asplayer_2 (Variables|Default|GetSpotLightSize))
  (Default|StartTimer _asplayer_2)
  (Utilities|FlowControl|DelayUntilNextTick)
  (Default|UpdateUI (Variables|/Game/KyleStuff/Player/Player.Player_C|GetUI _asplayer_2)))

(fn HighScore
  (params (CurrentScore :type Float%20%28double-precision%29))
  (if (> CurrentScore (Variables|Default|GetHighestPoints))
    (Variables|Default|SetHighestPoints CurrentScore)))

(fn PointCalculator
  (params (Difference :type Float%20%28double-precision%29) (CorrectPose :type Boolean) (CorrectMask :type Boolean))
  (return (Math|Float|Clamp(Float) (+ (Math|Float|Clamp(Float) (+ (* Difference -1.0) (Variables|Default|GetDistanceGenerosity)) -1e+03 0.0) (Variables|Default|GetMaxPoints) (* (Math|Conversions|ToFloat(Boolean) (not CorrectPose)) -3e+02) (* (Math|Conversions|ToFloat(Boolean) (not CorrectMask)) -3e+02)) 0.0 1e+03)))

(fn DifferenceCalculator
  (bind _asplayer (Utilities|Casting|CastToPlayer (Game|GetPlayerCharacter 0)))
  (return (+ (Math|Float|Absolute(Float) (Math|Vector|Distance(Vector) (Variables|/Game/KyleStuff/Player/Player.Player_C|GetTargetSpotlightPosition _asplayer) (Math|Vector|MakeVector 0.0 (.y (Transformation|GetActorLocation (Variables|/Game/KyleStuff/Player/Player.Player_C|GetSpotLight _asplayer))) (.z (Transformation|GetActorLocation (Variables|/Game/KyleStuff/Player/Player.Player_C|GetSpotLight _asplayer)))))) (Math|Float|Absolute(Float) (Math|Vector|Distance(Vector) (Variables|/Game/KyleStuff/Player/Player.Player_C|GetTargetPlayerPosition _asplayer) (Math|Vector|MakeVector (.x (Transformation|GetActorLocation _asplayer)) (.y (Transformation|GetActorLocation _asplayer)) 0.0))))))

(fn SetTarget
  (Variables|Default|SetTargetMask "NewEnumerator0")
  (Variables|Default|SetTargetPose "NewEnumerator4")
  (switch Utilities|FlowControl|Switch|SwitchonDifficulty (Variables|Default|GetDifficulty)
    (:NewEnumerator1
      _)
    (:NewEnumerator2
      (bind _output_get (Variables|Default|SetTargetMask (Utilities|Enum|ByteToEnumMasks (Math|Conversions|ToByte(Integer) (Math|Random|RandomInteger 3)))))))
  (bind _output_get_2 (Variables|Default|SetTargetPose (Utilities|Enum|ByteToEnumPoses (Math|Conversions|ToByte(Integer) (+ (Math|Random|RandomInteger 3) 1)))))
  (return _output_get _output_get_2))