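; Tree enemy that chases the first-person player and damages them at close range, destroying itself if the player's Start flag is off.
; Tick drives everything through a frame counter that times attacks, delayed removal and a walk animation faked by flipping Y scale.
; An active overlapping saw or a bullet kills it, enabling GeometryCollection physics, disabling some collision responses and adjusting the player's Chain, Timer and SawCooldown.
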(event OnComponentBeginOverlap(Overlap)
  (params (OverlappedComponent :type Primitive%20Component%20Object%20Reference) (OtherActor :type Actor%20Object%20Reference) (OtherComp :type Primitive%20Component%20Object%20Reference) (OtherBodyIndex :type Integer) (bFromSweep :type Boolean) (SweepResult :type Hit%20Result%20Structure%20%28by%20ref%29))
  (bind _capsule (Variables|Default|GetCapsule))
  (bind _capsule_2 (Variables|Default|GetCapsule))
  (bind _returnvalue (Transformation|GetWorldLocation _capsule_2))
  ;[1 1 1] Enemy Hit with Chainsaw or Bullet
  (if (Components|ComponentHasTag OtherComp "Saw")
    (Variables|Default|SetSawOverlapped true)
    (elif (Components|ComponentHasTag OtherComp "Bullet")
      ;[1 1 1] Enemy Death
      (if (not (> (Variables|Default|GetDeathTimer) 0.0))
        (Transformation|SetRelativeScale3D (Variables|Default|GetCapsule) "4.000000,4.000000,4.000000")
        (Physics|SetSimulatePhysics (Variables|Default|GetGeometryCollection) true)
        (Variables|Default|SetDeathTimer (+ (Variables|Default|GetEnemyTimer) 1.8e+02))
        ;[1 1 1] Death Sound
        (bind _output_get (Variables|Default|SetEnemySound (Math|Random|RandomInteger 3)))
        (if (== _output_get 0)
          (Audio|PlaySoundatLocation "/Game/Audio/TreeScream1.TreeScream1" _returnvalue "0, 0, 0" 0.5 1.0 0.0 0 0 0 0)
          (elif (== _output_get 1)
            (Audio|PlaySoundatLocation "/Game/Audio/TreeScream2.TreeScream2" _returnvalue "0, 0, 0" 0.5 1.0 0.0 0 0 0 0)
            (elif (== _output_get 2)
              (Audio|PlaySoundatLocation "/Game/Audio/TreeScream3.TreeScream3" _returnvalue "0, 0, 0" 0.5 1.0 0.0 0 0 0 0))))
        (Variables|/Game/Blueprints/BP_FirstPersonCharacter.BP_FirstPersonCharacter_C|SetChain (stale EventTick _asbp_first_person_character_2) (+ (Variables|/Game/Blueprints/BP_FirstPersonCharacter.BP_FirstPersonCharacter_C|GetChain (stale EventTick _asbp_first_person_character_2)) 1))
        (Variables|/Game/Blueprints/BP_FirstPersonCharacter.BP_FirstPersonCharacter_C|SetTimer (stale EventTick _asbp_first_person_character_2) (+ (Variables|/Game/Blueprints/BP_FirstPersonCharacter.BP_FirstPersonCharacter_C|GetTimer (stale EventTick _asbp_first_person_character_2)) -40))
        (Variables|/Game/Blueprints/BP_FirstPersonCharacter.BP_FirstPersonCharacter_C|SetSawCooldown (stale EventTick _asbp_first_person_character_2) (+ (Variables|/Game/Blueprints/BP_FirstPersonCharacter.BP_FirstPersonCharacter_C|GetSawCooldown (stale EventTick _asbp_first_person_character_2)) 30))
        (Collision|SetCollisionResponsetoChannel _capsule "ECC_Pawn" "ECR_Ignore")
        (Collision|SetCollisionResponsetoChannel (Variables|Default|GetOverlap) "ECC_PhysicsBody" "ECR_Ignore")
        (Collision|SetCollisionResponsetoChannel _capsule "ECC_GameTraceChannel1" "ECR_Ignore")))))

(event OnComponentEndOverlap(Overlap)
  (params (OverlappedComponent :type Primitive%20Component%20Object%20Reference) (OtherActor :type Actor%20Object%20Reference) (OtherComp :type Primitive%20Component%20Object%20Reference) (OtherBodyIndex :type Integer))
  ;[1 1 1] Enemy Hit with Chainsaw or Bullet
  (if (Components|ComponentHasTag OtherComp "Saw")
    (Variables|Default|SetSawOverlapped false)))

(event EventBeginPlay
  (bind _capsule (Variables|Default|GetCapsule))
  (bind _returnvalue (Transformation|GetWorldLocation _capsule))
  ;[1 1 1] Spawn Sound
  (if (== (Math|Random|RandomInteger 2) 0)
    (Audio|PlaySoundatLocation "/Game/Audio/TreeIdle1.TreeIdle1" _returnvalue "0, 0, 0" 0.1 1.0 0.0 0 0 0 0)
    (else
      (Audio|PlaySoundatLocation "/Game/Audio/TreeIdle2.TreeIdle2" _returnvalue "0, 0, 0" 0.1 1.0 0.0 0 0 0 0))))

(event EventTick
  (params (DeltaSeconds :type Float%20%28single-precision%29))
  (bind _capsule (Variables|Default|GetCapsule))
  (bind _capsule_2 (Variables|Default|GetCapsule))
  (bind _capsule_3 (Variables|Default|GetCapsule))
  (bind _returnvalue (Transformation|GetWorldLocation _capsule_3))
  ;[1 1 1] Enemy Rotation
  (bind _asbp_first_person_character (Utilities|Casting|CastToBP_FirstPersonCharacter (Game|Player|GetPlayerPawn 0)))
  (if (Variables|/Game/Blueprints/BP_FirstPersonCharacter.BP_FirstPersonCharacter_C|GetStart _asbp_first_person_character)
    (if (> (Variables|Default|GetDeathTimer) 0.0)
      _
      (else
        (Transformation|SetWorldRotation _capsule_3 (Math|Rotator|MakeRotator 0.0 0.0 (.Yaw (Math|Rotator|BreakRotator (Math|Rotator|FindLookatRotation _returnvalue (Transformation|GetWorldLocation (Variables|/Script/Engine.Character|GetCapsuleComponent _asbp_first_person_character)))))) false false)))
    ;[1 1 1] Enemy Movement
    (if (>= (Math|Vector|Distance(Vector) (Transformation|GetWorldLocation (Variables|/Script/Engine.Character|GetCapsuleComponent _asbp_first_person_character)) _returnvalue) 2.5e+02)
      (Transformation|AddWorldOffset _capsule_3 (* (Math|Vector|GetForwardVector _capsule_3) "10.000000,10.000000,0.000000") false false)
      (else
        ;[1 1 1] Enemy Attack and Player Hurt Sound
        (if (>= (Variables|Default|GetEnemyTimer) (Variables|Default|GetDamageTimer))
          (if (> (Variables|Default|GetDeathTimer) 0.0)
            _
            (else
              (Variables|/Game/Blueprints/BP_FirstPersonCharacter.BP_FirstPersonCharacter_C|SetHealth _asbp_first_person_character (- (Variables|/Game/Blueprints/BP_FirstPersonCharacter.BP_FirstPersonCharacter_C|GetHealth _asbp_first_person_character) 5))
              (Variables|Default|SetDamageTimer (+ (Variables|Default|GetEnemyTimer) 2e+01))
              (bind _output_get (Variables|Default|SetEnemySound (Math|Random|RandomInteger 4)))
              (if (== _output_get 0)
                (Audio|PlaySoundatLocation "/Game/Audio/Hurt1.Hurt1" _returnvalue "0, 0, 0" 1.0 1.0 0.0 0 0 0 0)
                (elif (== _output_get 1)
                  (Audio|PlaySoundatLocation "/Game/Audio/Hurt2.Hurt2" _returnvalue "0, 0, 0" 1.0 1.0 0.0 0 0 0 0)
                  (elif (== _output_get 2)
                    (Audio|PlaySoundatLocation "/Game/Audio/Hurt3.Hurt3" _returnvalue "0, 0, 0" 1.0 1.0 0.0 0 0 0 0)
                    (elif (== _output_get 3)
                      (Audio|PlaySoundatLocation "/Game/Audio/Attack2.Attack2" _returnvalue "0, 0, 0" 1.0 1.0 0.0 0 0 0 0))))))))))
    (if (>= (Variables|Default|GetEnemyTimer) (Variables|Default|GetAnimationTimer))
      (Variables|Default|SetAnimationTimer (+ (Variables|Default|GetEnemyTimer) 1e+01))
      (if (> (Variables|Default|GetDeathTimer) 0.0)
        _
        (else
          (Transformation|SetRelativeScale3D _capsule_2 (* (Transformation|GetWorldScale _capsule_2) "1.000000,-1.000000,1.000000")))))
    ;[1 1 1] Enemy Death
    (bind _asbp_first_person_character_2 (Utilities|Casting|CastToBP_FirstPersonCharacter (Game|Player|GetPlayerPawn 0)))
    (Variables|Default|SetEnemyTimer (+ (Variables|Default|GetEnemyTimer) 1.0))
    (if (> (Variables|Default|GetDeathTimer) 0.0)
      (if (>= (Variables|Default|GetEnemyTimer) (Variables|Default|GetDeathTimer))
        (Actor|DestroyActor)
        (else
          (if (Variables|/Game/Blueprints/BP_FirstPersonCharacter.BP_FirstPersonCharacter_C|GetSawDown _asbp_first_person_character_2) :!label _label
            (if (Variables|Default|GetSawOverlapped)
              (if (not (> (Variables|Default|GetDeathTimer) 0.0))
                (Transformation|SetRelativeScale3D _capsule_2 "4.000000,4.000000,4.000000")
                (Physics|SetSimulatePhysics (Variables|Default|GetGeometryCollection) true)
                (Variables|Default|SetDeathTimer (+ (Variables|Default|GetEnemyTimer) 1.8e+02))
                ;[1 1 1] Death Sound
                (bind _output_get_2 (Variables|Default|SetEnemySound (Math|Random|RandomInteger 3)))
                (if (== _output_get_2 0)
                  (Audio|PlaySoundatLocation "/Game/Audio/TreeScream1.TreeScream1" _returnvalue "0, 0, 0" 0.5 1.0 0.0 0 0 0 0)
                  (elif (== _output_get_2 1)
                    (Audio|PlaySoundatLocation "/Game/Audio/TreeScream2.TreeScream2" _returnvalue "0, 0, 0" 0.5 1.0 0.0 0 0 0 0)
                    (elif (== _output_get_2 2)
                      (Audio|PlaySoundatLocation "/Game/Audio/TreeScream3.TreeScream3" _returnvalue "0, 0, 0" 0.5 1.0 0.0 0 0 0 0))))
                (Variables|/Game/Blueprints/BP_FirstPersonCharacter.BP_FirstPersonCharacter_C|SetChain _asbp_first_person_character_2 (+ (Variables|/Game/Blueprints/BP_FirstPersonCharacter.BP_FirstPersonCharacter_C|GetChain _asbp_first_person_character_2) 1))
                (Variables|/Game/Blueprints/BP_FirstPersonCharacter.BP_FirstPersonCharacter_C|SetTimer _asbp_first_person_character_2 (+ (Variables|/Game/Blueprints/BP_FirstPersonCharacter.BP_FirstPersonCharacter_C|GetTimer _asbp_first_person_character_2) -40))
                (Variables|/Game/Blueprints/BP_FirstPersonCharacter.BP_FirstPersonCharacter_C|SetSawCooldown _asbp_first_person_character_2 (+ (Variables|/Game/Blueprints/BP_FirstPersonCharacter.BP_FirstPersonCharacter_C|GetSawCooldown _asbp_first_person_character_2) 30))
                (Collision|SetCollisionResponsetoChannel _capsule "ECC_Pawn" "ECR_Ignore")
                (Collision|SetCollisionResponsetoChannel (Variables|Default|GetOverlap) "ECC_PhysicsBody" "ECR_Ignore")
                (Collision|SetCollisionResponsetoChannel _capsule "ECC_GameTraceChannel1" "ECR_Ignore"))))))
      (else
        (goto _label)))
    (else
      (Actor|DestroyActor))))

(fn ConstructionScript)