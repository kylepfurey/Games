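; TreeEnemySpawn periodically spawns scaled-up TreeEnemy actors around the map and also drives the player's flashlight brightness.
; Each Tick reads the first-person character's state, setting the spotlight from its toggle and fading it after a late ElapsedTime threshold.
; Once Start is set, it rerolls random positions across frames until one is far enough from the player.
; It spawns there when ElapsedTime reaches SetTime, then schedules the next spawn.
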(event EventTick
  (params (DeltaSeconds :type Float%20%28single-precision%29))
  ;[1 1 1] Enemy Spawn
  (bind _asbp_first_person_character (Utilities|Casting|CastToBP_FirstPersonCharacter (Game|Player|GetPlayerPawn 0)))
  ;[1 1 1] Flashlight Out
  (if (>= (Variables|/Game/Blueprints/BP_FirstPersonCharacter.BP_FirstPersonCharacter_C|GetElapsedTime _asbp_first_person_character) 2.7e+03)
    (if (Variables|/Game/Blueprints/BP_FirstPersonCharacter.BP_FirstPersonCharacter_C|GetFlashlight _asbp_first_person_character)
      (Rendering|Components|Light|SetIntensity (Variables|/Game/Blueprints/BP_FirstPersonCharacter.BP_FirstPersonCharacter_C|GetSpotLight _asbp_first_person_character) (- 1.5e+04 (* (- (Variables|/Game/Blueprints/BP_FirstPersonCharacter.BP_FirstPersonCharacter_C|GetElapsedTime _asbp_first_person_character) 2.7e+03) 5e+01)))
      (else
        (Rendering|Components|Light|SetIntensity (Variables|/Game/Blueprints/BP_FirstPersonCharacter.BP_FirstPersonCharacter_C|GetSpotLight _asbp_first_person_character) 0.0 :!label _label)))
    (elif (Variables|/Game/Blueprints/BP_FirstPersonCharacter.BP_FirstPersonCharacter_C|GetFlashlight _asbp_first_person_character)
      (Rendering|Components|Light|SetIntensity (Variables|/Game/Blueprints/BP_FirstPersonCharacter.BP_FirstPersonCharacter_C|GetSpotLight _asbp_first_person_character) 1.5e+04)
      (else
        (goto _label))))
  (if (Variables|/Game/Blueprints/BP_FirstPersonCharacter.BP_FirstPersonCharacter_C|GetStart _asbp_first_person_character)
    (if (Variables|Default|GetReroll)
      (bind _output_get (Variables|Default|SetSpawnPosition (Math|Vector|MakeVector (+ (* (Math|Random|RandomFloat) 3564.0) -1.79e+03) (+ (* (Math|Random|RandomFloat) 3377.0) -1645.0) 1e+02)))
      (if (>= (Math|Float|Absolute(Float) (Math|Vector|Distance(Vector) _output_get (Transformation|GetWorldLocation (Variables|/Script/Engine.Character|GetCapsuleComponent _asbp_first_person_character)))) 1.2e+03)
        (Variables|Default|SetReroll false)
        (else
          (Variables|Default|SetReroll true :!label _label_2)))
      (elif (>= (Variables|/Game/Blueprints/BP_FirstPersonCharacter.BP_FirstPersonCharacter_C|GetElapsedTime _asbp_first_person_character) (Variables|Default|GetSetTime))
        (Game|SpawnActorfromClass "/Game/Blueprints/TreeEnemy.TreeEnemy_C" (Math|Transform|MakeTransform _output_get "0, 0, 0" "4.000000,4.000000,4.000000") "AlwaysSpawn" 0 0)
        (Variables|Default|SetSetTime (+ (Variables|/Game/Blueprints/BP_FirstPersonCharacter.BP_FirstPersonCharacter_C|GetElapsedTime _asbp_first_person_character) 45.0))
        (goto _label_2)))
    (else
      (Variables|Default|SetSetTime 0.0))))

(fn ConstructionScript)