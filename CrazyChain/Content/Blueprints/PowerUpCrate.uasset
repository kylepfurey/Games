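; Breakable power-up crate that spawns a PowerUp when shot by a bullet or cut by the player's chainsaw.
; Tagged overlaps detect hits, with saw hits also requiring the player's SawDown flag.
; Breaking enables Geometry Collection physics and relaxes selected collision responses.
; A Tick-counted timer removes broken crates after a short delay and untouched ones after a longer lifetime, or immediately when the player's Start flag is false.
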(event OnComponentBeginOverlap(Overlap)
  (params (OverlappedComponent :type Primitive%20Component%20Object%20Reference) (OtherActor :type Actor%20Object%20Reference) (OtherComp :type Primitive%20Component%20Object%20Reference) (OtherBodyIndex :type Integer) (bFromSweep :type Boolean) (SweepResult :type Hit%20Result%20Structure%20%28by%20ref%29))
  (bind _box (Variables|Default|GetBox))
  ;[1 1 1] Crate Item Hit with Chainsaw or Bullet
  (if (Components|ComponentHasTag OtherComp "Saw")
    (Variables|Default|SetSawOverlapped true)
    (elif (Components|ComponentHasTag OtherComp "Bullet")
      ;[1 1 1] Crate
      (if (not (> (Variables|Default|GetDeathTimer) 0.0))
        (Physics|SetSimulatePhysics (Variables|Default|GetGeometryCollection) true)
        (Physics|SetSimulatePhysics _box false)
        (Variables|Default|SetDeathTimer (+ (Variables|Default|GetCrateTimer) 1.8e+02))
        (Collision|SetCollisionResponsetoChannel _box "ECC_Pawn" "ECR_Ignore")
        (Collision|SetCollisionResponsetoChannel _box "ECC_Destructible" "ECR_Ignore")
        (Collision|SetCollisionResponsetoChannel _box "ECC_GameTraceChannel1" "ECR_Ignore")
        (Game|SpawnActorfromClass "/Game/Blueprints/PowerUp.PowerUp_C" (Transformation|GetWorldTransform _box) "AlwaysSpawn" 0 0)))))

(event OnComponentEndOverlap(Overlap)
  (params (OverlappedComponent :type Primitive%20Component%20Object%20Reference) (OtherActor :type Actor%20Object%20Reference) (OtherComp :type Primitive%20Component%20Object%20Reference) (OtherBodyIndex :type Integer))
  ;[1 1 1] Crate Item Hit with Chainsaw or Bullet
  (if (Components|ComponentHasTag OtherComp "Saw")
    (Variables|Default|SetSawOverlapped false)))

(event EventTick
  (params (DeltaSeconds :type Float%20%28single-precision%29))
  (bind _box (Variables|Default|GetBox))
  ;[1 1 1] Crate
  (bind _asbp_first_person_character (Utilities|Casting|CastToBP_FirstPersonCharacter (Game|GetPlayerCharacter 0)))
  (if (Variables|/Game/Blueprints/BP_FirstPersonCharacter.BP_FirstPersonCharacter_C|GetStart _asbp_first_person_character)
    (Variables|Default|SetCrateTimer (+ (Variables|Default|GetCrateTimer) 1.0))
    (if (> (Variables|Default|GetDeathTimer) 0.0)
      (if (>= (Variables|Default|GetCrateTimer) (Variables|Default|GetDeathTimer))
        (Actor|DestroyActor :!label _label)
        (else
          (if (Variables|/Game/Blueprints/BP_FirstPersonCharacter.BP_FirstPersonCharacter_C|GetSawDown _asbp_first_person_character) :!label _label_2
            (if (Variables|Default|GetSawOverlapped)
              (if (not (> (Variables|Default|GetDeathTimer) 0.0))
                (Physics|SetSimulatePhysics (Variables|Default|GetGeometryCollection) true)
                (Physics|SetSimulatePhysics _box false)
                (Variables|Default|SetDeathTimer (+ (Variables|Default|GetCrateTimer) 1.8e+02))
                (Collision|SetCollisionResponsetoChannel _box "ECC_Pawn" "ECR_Ignore")
                (Collision|SetCollisionResponsetoChannel _box "ECC_Destructible" "ECR_Ignore")
                (Collision|SetCollisionResponsetoChannel _box "ECC_GameTraceChannel1" "ECR_Ignore")
                (Game|SpawnActorfromClass "/Game/Blueprints/PowerUp.PowerUp_C" (Transformation|GetWorldTransform _box) "AlwaysSpawn" 0 0))))))
      (elif (and (>= (Variables|Default|GetCrateTimer) 9e+02) (== (Variables|Default|GetDeathTimer) 0.0))
        (goto _label)
        (else
          (goto _label_2))))
    (else
      (goto _label))))

(fn ConstructionScript)