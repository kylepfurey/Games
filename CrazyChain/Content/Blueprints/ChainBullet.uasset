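; ChainBullet is a projectile actor with a spinning chain visual that destroys itself when it hits a component tagged Destructible.
; On BeginPlay the chain gets a random starting pitch and randomly takes either the standard or gold chain material.
; Each Tick spins the chain and advances a frame counter that destroys the actor after a fixed count, so lifetime depends on frame rate.
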(event OnComponentBeginOverlap(Collision)
  (params (OverlappedComponent :type Primitive%20Component%20Object%20Reference) (OtherActor :type Actor%20Object%20Reference) (OtherComp :type Primitive%20Component%20Object%20Reference) (OtherBodyIndex :type Integer) (bFromSweep :type Boolean) (SweepResult :type Hit%20Result%20Structure%20%28by%20ref%29))
  ;[1 1 1] Destroy on Hit
  (if (Components|ComponentHasTag OtherComp "Destructible")
    (Actor|DestroyActor)))

(event EventTick
  (params (DeltaSeconds :type Float%20%28single-precision%29))
  ;[1 1 1] Destroy Bullet
  (Variables|Default|SetDeathTimer (+ (Variables|Default|GetDeathTimer) 1.0))
  (if (>= (Variables|Default|GetDeathTimer) 1.5e+02)
    (Actor|DestroyActor)
    (else
      ;[1 1 1] Rotation and Color of Chain
      (Transformation|AddRelativeRotation (Variables|Default|GetChain) "120.000000,0.000000,0.000000" false false))))

(event EventBeginPlay
  (bind _chain (Variables|Default|GetChain))
  ;[1 1 1] Rotation and Color of Chain
  (Transformation|AddRelativeRotation (Variables|Default|GetChain) (Math|Rotator|MakeRotator 0.0 (* (Math|Random|RandomFloat) 3.6e+02) 0.0) false false)
  (if (== (Math|Random|RandomInteger 2) 1)
    (Rendering|Material|SetMaterial _chain 0 "/Game/Assets/Chain/Mat_Chain.Mat_Chain")
    (else
      (Rendering|Material|SetMaterial _chain 0 "/Game/Assets/Chain/Mat_Chain_Gold.Mat_Chain_Gold"))))

(fn ConstructionScript)