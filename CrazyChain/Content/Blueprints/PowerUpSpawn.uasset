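; PowerUpSpawn periodically spawns a scaled-up PowerUpCrate at a random ground-area position, facing the player.
; On Tick, once the first-person character's Start flag is set, it rerolls positions within fixed bounds until one lies far enough from the player.
; It then waits for the character's ElapsedTime to reach SetTime, spawns the crate, advances the threshold by a fixed interval and rerolls.
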(event EventTick
  (params (DeltaSeconds :type Float%20%28single-precision%29))
  ;[1 1 1] Enemy Spawn
  (bind _asbp_first_person_character (Utilities|Casting|CastToBP_FirstPersonCharacter (Game|Player|GetPlayerPawn 0)))
  (if (Variables|/Game/Blueprints/BP_FirstPersonCharacter.BP_FirstPersonCharacter_C|GetStart _asbp_first_person_character)
    (if (Variables|Default|GetReroll)
      (bind _output_get (Variables|Default|SetSpawnPosition (Math|Vector|MakeVector (+ (* (Math|Random|RandomFloat) 3564.0) -1.79e+03) (+ (* (Math|Random|RandomFloat) 3377.0) -1645.0) 1e+01)))
      (if (>= (Math|Float|Absolute(Float) (Math|Vector|Distance(Vector) _output_get (Transformation|GetWorldLocation (Variables|/Script/Engine.Character|GetCapsuleComponent _asbp_first_person_character)))) 8.5e+02)
        (Variables|Default|SetReroll false)
        (else
          (Variables|Default|SetReroll true :!label _label)))
      (elif (>= (Variables|/Game/Blueprints/BP_FirstPersonCharacter.BP_FirstPersonCharacter_C|GetElapsedTime _asbp_first_person_character) (Variables|Default|GetSetTime))
        (Game|SpawnActorfromClass "/Game/Blueprints/PowerUpCrate.PowerUpCrate_C" (Math|Transform|MakeTransform _output_get (Math|Rotator|FindLookatRotation _output_get (Transformation|GetWorldLocation (Variables|/Script/Engine.Character|GetCapsuleComponent _asbp_first_person_character))) "2.500000,2.500000,2.500000") "AlwaysSpawn" 0 0)
        (Variables|Default|SetSetTime (+ (Variables|/Game/Blueprints/BP_FirstPersonCharacter.BP_FirstPersonCharacter_C|GetElapsedTime _asbp_first_person_character) 4.5e+02))
        (goto _label)))
    (else
      (Variables|Default|SetSetTime 4.5e+02))))

(fn ConstructionScript)