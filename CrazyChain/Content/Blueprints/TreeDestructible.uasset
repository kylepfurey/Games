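; Destructible tree that breaks when a "Saw"-tagged component overlaps it, and resets between games.
; The overlap checks the player's saw state (skipped at zero ChainGunAmmo), then enables GeometryCollection physics and ignores several collision channels.
; Tick pins the capsule in place and shrinks the broken pieces until it destroys them.
; Tick also arms Reset while the player's Start flag is false, then replaces the actor with a fresh copy when Start turns true.
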(event OnComponentBeginOverlap(Overlap)
  (params (OverlappedComponent :type Primitive%20Component%20Object%20Reference) (OtherActor :type Actor%20Object%20Reference) (OtherComp :type Primitive%20Component%20Object%20Reference) (OtherBodyIndex :type Integer) (bFromSweep :type Boolean) (SweepResult :type Hit%20Result%20Structure%20%28by%20ref%29))
  (bind _capsule (Variables|Default|GetCapsule))
  ;[1 1 1] Tree Hit with Chainsaw
  (if (Utilities|IsValid (Variables|Default|GetGeometryCollection))
    (if (Components|ComponentHasTag OtherComp "Saw")
      (bind _asbp_first_person_character (Utilities|Casting|CastToBP_FirstPersonCharacter (Game|Player|GetPlayerPawn 0)))
      (if (> (Variables|/Game/Blueprints/BP_FirstPersonCharacter.BP_FirstPersonCharacter_C|GetChainGunAmmo _asbp_first_person_character) 0)
        (if (Variables|/Game/Blueprints/BP_FirstPersonCharacter.BP_FirstPersonCharacter_C|GetSawDown _asbp_first_person_character)
          (Physics|SetSimulatePhysics (Variables|Default|GetGeometryCollection) true :!label _label)
          (Collision|SetCollisionResponsetoChannel _capsule "ECC_Pawn" "ECR_Ignore")
          (Collision|SetCollisionResponsetoChannel _capsule "ECC_PhysicsBody" "ECR_Ignore")
          (Collision|SetCollisionResponsetoChannel _capsule "ECC_GameTraceChannel1" "ECR_Ignore")
          (Variables|Default|SetOverlapping true))
        (else
          (goto _label))))))

(event EventBeginPlay
  (bind _capsule (Variables|Default|GetCapsule))
  ;[1 1 1] Reset Tree on Game End
  (bind _output_get (Variables|Default|SetStartingPosition (Transformation|GetWorldLocation _capsule)))
  (bind _output_get_2 (Variables|Default|SetStartingRotation (Transformation|GetWorldRotation _capsule)))
  (Variables|Default|SetReset false))

(event EventTick
  (params (DeltaSeconds :type Float%20%28single-precision%29))
  (bind _geometrycollection (Variables|Default|GetGeometryCollection))
  (bind _returnvalue (Transformation|GetWorldScale _geometrycollection))
  ;[1 1 1] Reset Tree on Game End
  (Transformation|SetWorldLocationAndRotation (Variables|Default|GetCapsule) (stale EventBeginPlay _output_get) (stale EventBeginPlay _output_get_2) false false)
  (bind _asbp_first_person_character (Utilities|Casting|CastToBP_FirstPersonCharacter (Game|Player|GetPlayerPawn 0)))
  (if (Variables|Default|GetOverlapping)
    (if (Utilities|IsValid (Variables|Default|GetGeometryCollection))
      (Transformation|SetWorldScale3D _geometrycollection (- _returnvalue "0.001500,0.001500,0.001500"))
      (if (Utilities|Operators|EqualEqual _returnvalue "0.100000,0.100000,0.100000" 0.1)
        (if (Utilities|IsValid (Variables|Default|GetGeometryCollection))
          (Components|DestroyComponent (Variables|Default|GetGeometryCollection)))
        (else
          (if (Variables|/Game/Blueprints/BP_FirstPersonCharacter.BP_FirstPersonCharacter_C|GetStart _asbp_first_person_character) :!label _label
            (if (Variables|Default|GetReset)
              (Game|SpawnActorfromClass "TreeDestructible_C" (Math|Transform|MakeTransform (stale EventBeginPlay _output_get) (stale EventBeginPlay _output_get_2)) "AlwaysSpawn" 0 0)
              (Actor|DestroyActor))
            (elif (not (Variables|Default|GetReset))
              (Variables|Default|SetReset true)))))
      (else
        (goto _label)))
    (else
      (goto _label))))

(fn ConstructionScript)