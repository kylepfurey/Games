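; A timed pickup actor that randomly becomes one of four power-ups on BeginPlay: health, timer, speed or chain.
; Tick spins the box, sets the matching material and destroys the actor after 300 frames, or immediately if the first-person character's Start flag is off.
; Overlap by a component tagged "Player" copies the power-up index to that character and destroys the pickup, leaving the effect to the character.
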(event OnComponentBeginOverlap(Box)
  (params (OverlappedComponent :type Primitive%20Component%20Object%20Reference) (OtherActor :type Actor%20Object%20Reference) (OtherComp :type Primitive%20Component%20Object%20Reference) (OtherBodyIndex :type Integer) (bFromSweep :type Boolean) (SweepResult :type Hit%20Result%20Structure%20%28by%20ref%29))
  ;[1 1 1] Player Grabs Item
  (bind _asbp_first_person_character (Utilities|Casting|CastToBP_FirstPersonCharacter (Game|Player|GetPlayerPawn 0)))
  (if (Components|ComponentHasTag OtherComp "Player")
    (Variables|/Game/Blueprints/BP_FirstPersonCharacter.BP_FirstPersonCharacter_C|SetPowerUp _asbp_first_person_character (Variables|Default|GetPowerUp))
    (Actor|DestroyActor)))

(event EventTick
  (params (DeltaSeconds :type Float%20%28single-precision%29))
  (bind _staticmesh (Variables|Default|GetStaticMesh))
  (bind _box (Variables|Default|GetBox))
  ;[1 1 1] Set Position, Material, and Rotate Item
  ;[1 1 1] Set Item and Deletion
  (bind _asbp_first_person_character (Utilities|Casting|CastToBP_FirstPersonCharacter (Game|Player|GetPlayerPawn 0)))
  (if (Variables|/Game/Blueprints/BP_FirstPersonCharacter.BP_FirstPersonCharacter_C|GetStart _asbp_first_person_character)
    (Variables|Default|SetItemTimer (+ (Variables|Default|GetItemTimer) 1.0))
    (Transformation|SetWorldRotation _box (Math|Rotator|MakeRotator 0.0 0.0 (+ (.Yaw (Math|Rotator|BreakRotator (Transformation|GetWorldRotation _box))) 5.0)) false false)
    ;[1 1 1] Player Grabs Item
    (if (Utilities|IsValid _staticmesh)
      (if (== (Variables|Default|GetPowerUp) 1)
        (Rendering|Material|SetMaterial _staticmesh 0 "/Game/Assets/PowerUps/healthpowerup_Mat.healthpowerup_Mat")
        (elif (== (Variables|Default|GetPowerUp) 2)
          (Rendering|Material|SetMaterial _staticmesh 0 "/Game/Assets/PowerUps/timerpowerup_Mat.timerpowerup_Mat")
          (elif (== (Variables|Default|GetPowerUp) 3)
            (Rendering|Material|SetMaterial _staticmesh 0 "/Game/Assets/PowerUps/speedpowerup_Mat.speedpowerup_Mat")
            (elif (== (Variables|Default|GetPowerUp) 4)
              (Rendering|Material|SetMaterial _staticmesh 0 "/Game/Assets/PowerUps/chainpowerup_Mat.chainpowerup_Mat")))))
      (if (>= (Variables|Default|GetItemTimer) 3e+02)
        (Actor|DestroyActor :!label _label))
      (else
        (goto _label)))
    (else
      (goto _label))))

(event EventBeginPlay
  ;[1 1 1] Set Item and Deletion
  (Variables|Default|SetPowerUp (+ (Math|Random|RandomInteger 4) 1)))

(fn ConstructionScript)