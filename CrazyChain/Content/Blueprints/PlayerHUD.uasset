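; Player HUD for a first-person chain-themed game jam title, drawing the title screen, gameplay stats and game-over screen.
; DrawHUD polls BP_FirstPersonCharacter for health, chains, timers, crosshair and ammo or saw cooldown, layering offset text as drop shadows.
; Tick advances the logo fade, sets TitleOver and exits the title on Start.
; BeginPlay schedules title audio; gameplay drawing requires that music component, which it mutes.
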(event EventTick
  (params (DeltaSeconds :type Float%20%28single-precision%29))
  ;[1 1 1] Title Screen
  (if (>= 15.75 (Variables|Default|GetFadeTimer))
    (Variables|Default|SetFadeTimer (+ 0.09 (Variables|Default|GetFadeTimer))))
  (bind _asbp_first_person_character (Utilities|Casting|CastToBP_FirstPersonCharacter (Game|GetPlayerCharacter 0)))
  (Variables|/Game/Blueprints/BP_FirstPersonCharacter.BP_FirstPersonCharacter_C|SetTitleOver _asbp_first_person_character (not (>= 15.75 (Variables|Default|GetFadeTimer))))
  (if (Variables|Default|GetOpening)
    (if (Variables|/Game/Blueprints/BP_FirstPersonCharacter.BP_FirstPersonCharacter_C|GetStart _asbp_first_person_character)
      (Variables|Default|SetOpening false))))

(event EventBeginPlay
  ;[1 1 1] Game Beginning with Sounds
  (bind _returnvalue (AddComponent|AddGameplayTasksComponent))
  (GameplayTasks|TaskWaitDelay _returnvalue 0.25
    (:then
      (GameplayTasks|TaskWaitDelay _returnvalue 5.25
        (:OnFinish
          (bind _returnvalue_2 (Audio|SpawnSoundatLocation "/Game/Audio/TitleScreen.TitleScreen" "0, 0, 0" "0, 0, 0" 0.5 1.0 0.0 0 0)))))
    (:OnFinish
      (Audio|SpawnSoundatLocation "/Game/Audio/Title.Title" "0, 0, 0" "0, 0, 0" 1e+01 1.0 0.0 0 0))))

(event EventDrawHUD
  (params (SizeX :type Integer) (SizeY :type Integer))
  (bind _fadetimer (Variables|Default|GetFadeTimer))
  (bind _returnvalue (- 15.75 _fadetimer))
  ;[1 1 1] Draw HUD
  (Variables|Default|SetSizeX (Math|Conversions|ToFloat(Integer) (/ SizeX 2)))
  (Variables|Default|SetSizeY (Math|Conversions|ToFloat(Integer) (/ SizeY 2)))
  (bind _asbp_first_person_character (Utilities|Casting|CastToBP_FirstPersonCharacter (Game|GetPlayerCharacter 0)))
  ;[1 1 1] Title Screen
  (if (Variables|Default|GetOpening)
    (Class|HUD|DrawTextureSimple "/Game/Assets/HUD/crazychain.crazychain" (+ (Variables|Default|GetSizeX) -505.0) (+ (Variables|Default|GetSizeY) -3e+02) 0.5 false)
    (HUD|DrawText "Programmed by Kyle and Chris, Art and Models by Avery, Sounds and Music by Shea, and Theme by Jaleel. Made for 2023 SNHU Game Jam." "(R=0.000000,G=0.000000,B=0.000000,A=1.000000)" (+ (Variables|Default|GetSizeX) -5.9e+02) (+ (+ (* (Variables|Default|GetSizeY) 2.0) -75.0) 2.0) 0 1.5 false)
    (HUD|DrawText "Programmed by Kyle and Chris, Art and Models by Avery, Sounds and Music by Shea, and Theme by Jaleel. Made for 2023 SNHU Game Jam." "(R=1.000000,G=1.000000,B=1.000000,A=1.000000)" (+ (Variables|Default|GetSizeX) -592.0) (+ (* (Variables|Default|GetSizeY) 2.0) -75.0) 0 1.5 false)
    (HUD|DrawText "Press Space to Start" "(R=0.000000,G=0.000000,B=0.000000,A=1.000000)" (+ (Variables|Default|GetSizeX) -2.2e+02) (+ (+ (+ (Variables|Default|GetSizeY) -3e+02) 535.0) 2.0) 0 3.5 false)
    (HUD|DrawText "Press Space to Start" "(R=1.000000,G=1.000000,B=1.000000,A=1.000000)" (+ (Variables|Default|GetSizeX) -222.0) (+ (+ (Variables|Default|GetSizeY) -3e+02) 535.0) 0 3.5 false)
    ;[1 1 1] Game Beginning with Sounds
    (HUD|DrawRect (Math|Color|MakeColor 0.0 0.0 0.0 _returnvalue) 0.0 0.0 (Math|Conversions|ToFloat(Integer) SizeX) (Math|Conversions|ToFloat(Integer) SizeY))
    (if (>= _returnvalue 1.0)
      (Class|HUD|DrawTextureSimple "/Game/Assets/HUD/Crowbyte_Logo_Chainsaw.Crowbyte_Logo_Chainsaw" (+ (Variables|Default|GetSizeX) -4e+02) (+ (Variables|Default|GetSizeY) -375.0) 1.5 false))
    (elif (Utilities|IsValid (stale EventBeginPlay _returnvalue_2))
      (Audio|Components|Audio|SetVolumeMultiplier (stale EventBeginPlay _returnvalue_2) 0.0 :!class /Script/Engine.AudioComponent)
      ;[1 1 1] HUD
      (Class|HUD|DrawTextureSimple "/Game/Assets/HUD/chains.chains" (+ (* (Variables|Default|GetSizeX) 0.0) 3e+01) (+ (* (Variables|Default|GetSizeY) 2.0) -1.4e+02) 0.15 false)
      (HUD|DrawText (Utilities|String|ToString(Integer) (Variables|/Game/Blueprints/BP_FirstPersonCharacter.BP_FirstPersonCharacter_C|GetChain _asbp_first_person_character)) "(R=0.000000,G=0.000000,B=0.000000,A=1.000000)" (+ (* (Variables|Default|GetSizeX) 0.0) 342.0) (+ (* (Variables|Default|GetSizeY) 2.0) -98.0) 0 5.0 false)
      (HUD|DrawText (Utilities|String|ToString(Integer) (Variables|/Game/Blueprints/BP_FirstPersonCharacter.BP_FirstPersonCharacter_C|GetChain _asbp_first_person_character)) "(R=0.879622,G=0.760525,B=0.000000,A=1.000000)" (+ (* (Variables|Default|GetSizeX) 0.0) 3.4e+02) (+ (* (Variables|Default|GetSizeY) 2.0) -1e+02) 0 5.0 false)
      (Class|HUD|DrawTextureSimple "/Game/Assets/HUD/health.health" (+ (* (Variables|Default|GetSizeX) 0.0) 3e+01) (+ (* (Variables|Default|GetSizeY) 2.0) -2.1e+02) 0.147 false)
      (HUD|DrawText (Utilities|String|ToString(Integer) (Variables|/Game/Blueprints/BP_FirstPersonCharacter.BP_FirstPersonCharacter_C|GetHealth _asbp_first_person_character)) "(R=0.000000,G=0.000000,B=0.000000,A=1.000000)" (+ (* (Variables|Default|GetSizeX) 0.0) 342.0) (+ (* (Variables|Default|GetSizeY) 2.0) -168.0) 0 5.0 false)
      (HUD|DrawText (Utilities|String|ToString(Integer) (Variables|/Game/Blueprints/BP_FirstPersonCharacter.BP_FirstPersonCharacter_C|GetHealth _asbp_first_person_character)) "(R=1.000000,G=0.000000,B=0.000000,A=1.000000)" (+ (* (Variables|Default|GetSizeX) 0.0) 3.4e+02) (+ (* (Variables|Default|GetSizeY) 2.0) -1.7e+02) 0 5.0 false)
      (HUD|DrawText (Utilities|String|Append ":   " (Utilities|String|ToString(Integer) (Variables|/Game/Blueprints/BP_FirstPersonCharacter.BP_FirstPersonCharacter_C|GetHighestChain _asbp_first_person_character))) "(R=0.000000,G=0.000000,B=0.000000,A=1.000000)" (+ (* (Variables|Default|GetSizeX) 0.0) 462.0) (+ (* (Variables|Default|GetSizeY) 2.0) -98.0) 0 5.0 false)
      (HUD|DrawText (Utilities|String|Append ":   " (Utilities|String|ToString(Integer) (Variables|/Game/Blueprints/BP_FirstPersonCharacter.BP_FirstPersonCharacter_C|GetHighestChain _asbp_first_person_character))) "(R=0.000000,G=0.250000,B=1.000000,A=1.000000)" (+ (* (Variables|Default|GetSizeX) 0.0) 4.6e+02) (+ (* (Variables|Default|GetSizeY) 2.0) -1e+02) 0 5.0 false)
      (HUD|DrawText (Utilities|String|ToString(Float) (/ (Math|Conversions|ToFloat(Integer) (Math|Float|Round (/ (- 3e+02 (Math|Conversions|ToFloat(Integer) (Variables|/Game/Blueprints/BP_FirstPersonCharacter.BP_FirstPersonCharacter_C|GetTimer _asbp_first_person_character))) 3.0))) 1e+01)) "(R=0.000000,G=0.000000,B=0.000000,A=1.000000)" (+ (Variables|Default|GetSizeX) -48.0) (+ (* (Variables|Default|GetSizeY) 2.0) -98.0) 0 5.0 false)
      (HUD|DrawText (Utilities|String|ToString(Float) (/ (Math|Conversions|ToFloat(Integer) (Math|Float|Round (/ (- 3e+02 (Math|Conversions|ToFloat(Integer) (Variables|/Game/Blueprints/BP_FirstPersonCharacter.BP_FirstPersonCharacter_C|GetTimer _asbp_first_person_character))) 3.0))) 1e+01)) "(R=0.093059,G=1.000000,B=0.093059,A=1.000000)" (+ (Variables|Default|GetSizeX) -5e+01) (+ (* (Variables|Default|GetSizeY) 2.0) -1e+02) 0 5.0 false)
      (HUD|DrawText (Utilities|String|ToString(Float) (/ (Math|Conversions|ToFloat(Integer) (Math|Float|Round (/ (Variables|/Game/Blueprints/BP_FirstPersonCharacter.BP_FirstPersonCharacter_C|GetElapsedTime _asbp_first_person_character) 3.0))) 1e+01)) "(R=0.000000,G=0.000000,B=0.000000,A=1.000000)" (+ (Variables|Default|GetSizeX) -18.0) (+ (* (Variables|Default|GetSizeY) 0.0) 32.0) 0 1.3 false)
      (HUD|DrawText (Utilities|String|ToString(Float) (/ (Math|Conversions|ToFloat(Integer) (Math|Float|Round (/ (Variables|/Game/Blueprints/BP_FirstPersonCharacter.BP_FirstPersonCharacter_C|GetElapsedTime _asbp_first_person_character) 3.0))) 1e+01)) "(R=0.480314,G=1.000000,B=0.000000,A=1.000000)" (+ (Variables|Default|GetSizeX) -2e+01) (+ (* (Variables|Default|GetSizeY) 0.0) 3e+01) 0 1.3 false)
      (if (Variables|/Game/Blueprints/BP_FirstPersonCharacter.BP_FirstPersonCharacter_C|GetCrosshair _asbp_first_person_character)
        (Class|HUD|DrawTextureSimple "/Game/Assets/HUD/crosshair2.crosshair2" (+ (Variables|Default|GetSizeX) -13.75) (+ (Variables|Default|GetSizeY) -15.0) 0.025 false)
        (else
          (Class|HUD|DrawTextureSimple "/Game/Assets/HUD/crosshair.crosshair" (+ (Variables|Default|GetSizeX) -13.75) (+ (Variables|Default|GetSizeY) -15.0) 0.025 false)))
      (if (> (Variables|/Game/Blueprints/BP_FirstPersonCharacter.BP_FirstPersonCharacter_C|GetChainGunAmmo _asbp_first_person_character) 0)
        (HUD|DrawText (Utilities|String|ToString(Integer) (Math|Float|Round (/ (Math|Conversions|ToFloat(Integer) (Variables|/Game/Blueprints/BP_FirstPersonCharacter.BP_FirstPersonCharacter_C|GetChainGunAmmo _asbp_first_person_character)) 1.0))) "(R=1.000000,G=1.000000,B=1.000000,A=1.000000)" (+ (* (Variables|Default|GetSizeX) 2.0) -248.0) (+ (* (Variables|Default|GetSizeY) 2.0) -158.0) 0 1e+01 false)
        (HUD|DrawText (Utilities|String|ToString(Integer) (Math|Float|Round (/ (Math|Conversions|ToFloat(Integer) (Variables|/Game/Blueprints/BP_FirstPersonCharacter.BP_FirstPersonCharacter_C|GetChainGunAmmo _asbp_first_person_character)) 1.0))) "(R=0.000000,G=0.571125,B=1.000000,A=1.000000)" (+ (* (Variables|Default|GetSizeX) 2.0) -2.5e+02) (+ (* (Variables|Default|GetSizeY) 2.0) -1.6e+02) 0 1e+01 false)
        (else
          (HUD|DrawText (Utilities|String|ToString(Integer) (Math|Float|Round (/ (Math|Conversions|ToFloat(Integer) (Variables|/Game/Blueprints/BP_FirstPersonCharacter.BP_FirstPersonCharacter_C|GetSawCooldown _asbp_first_person_character)) 1.0))) "(R=1.000000,G=1.000000,B=1.000000,A=1.000000)" (+ (* (Variables|Default|GetSizeX) 2.0) -248.0) (+ (* (Variables|Default|GetSizeY) 2.0) -158.0) 0 1e+01 false)
          (if (> (Variables|/Game/Blueprints/BP_FirstPersonCharacter.BP_FirstPersonCharacter_C|GetBoostTimer _asbp_first_person_character) (Variables|/Game/Blueprints/BP_FirstPersonCharacter.BP_FirstPersonCharacter_C|GetElapsedTime _asbp_first_person_character))
            (HUD|DrawText (Utilities|String|ToString(Integer) (Math|Float|Round (/ (Math|Conversions|ToFloat(Integer) (Variables|/Game/Blueprints/BP_FirstPersonCharacter.BP_FirstPersonCharacter_C|GetSawCooldown _asbp_first_person_character)) 1.0))) "(R=1.000000,G=0.080220,B=0.904661,A=1.000000)" (+ (* (Variables|Default|GetSizeX) 2.0) -2.5e+02) (+ (* (Variables|Default|GetSizeY) 2.0) -1.6e+02) 0 1e+01 false)
            (else
              (HUD|DrawText (Utilities|String|ToString(Integer) (Math|Float|Round (/ (Math|Conversions|ToFloat(Integer) (Variables|/Game/Blueprints/BP_FirstPersonCharacter.BP_FirstPersonCharacter_C|GetSawCooldown _asbp_first_person_character)) 1.0))) "(R=1.000000,G=0.107647,B=0.000000,A=1.000000)" (+ (* (Variables|Default|GetSizeX) 2.0) -2.5e+02) (+ (* (Variables|Default|GetSizeY) 2.0) -1.6e+02) 0 1e+01 false)))))
      ;[1 1 1] Game Over
      (if (not (Variables|/Game/Blueprints/BP_FirstPersonCharacter.BP_FirstPersonCharacter_C|GetStart _asbp_first_person_character))
        (Class|HUD|DrawTextureSimple "/Game/Assets/HUD/gameover.gameover" (+ (Variables|Default|GetSizeX) -505.0) (+ (Variables|Default|GetSizeY) -275.0) 0.5 false)
        (HUD|DrawText "Press Space to Start" "(R=0.000000,G=0.000000,B=0.000000,A=1.000000)" (+ (Variables|Default|GetSizeX) -2.2e+02) (+ (+ (+ (Variables|Default|GetSizeY) -275.0) 5.1e+02) 2.0) 0 3.5 false)
        (HUD|DrawText "Press Space to Start" "(R=1.000000,G=1.000000,B=1.000000,A=1.000000)" (+ (Variables|Default|GetSizeX) -222.0) (+ (+ (Variables|Default|GetSizeY) -275.0) 5.1e+02) 0 3.5 false)))))

(fn ConstructionScript)